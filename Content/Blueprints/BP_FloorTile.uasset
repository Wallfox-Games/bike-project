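; BP_FloorTile is a track segment for an endlessly spawned level with three obstacle lanes.
; Construction picks a random child tile from BP_LevelDatabaseActor and, in Checker mode, adds lane-indexed BP_ObstacleChecker actors at the spawn points.
; GetAttachTransform exposes the attach point's world transform.
; When the player hits EndTrigger, it calls the game mode's NextFloorTile, then after a delay destroys itself and calls DestroyBuildings on BP_Buildings.
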(event `self.ReceiveBeginPlay`
  (bind _returnvalue (`GameplayStatics.GetActorOfClass` "/Game/Blueprints/Art/BP_Buildings.BP_Buildings_C"))
  (set `self.Building Reference` _returnvalue))

(event `self.EndTrigger.OnComponentBeginOverlap`
  (params (OverlappedComponent :type "PrimitiveComponent Object Reference") (OtherActor :type "Actor Object Reference") (OtherComp :type "PrimitiveComponent Object Reference") (OtherBodyIndex :type Integer) (bFromSweep :type Boolean) (SweepResult :type "HitResult Structure (by ref)"))
  (cast `/Game/Blueprints/BP_PlayerCharacter` OtherActor)
  (bind _asbp_bike_project_game_mode_base (cast `/Game/Blueprints/BP_BikeProjectGameModeBase` (`GameplayStatics.GetGameMode`)))
  (`/Game/Blueprints/BP_BikeProjectGameModeBase.Next Floor Tile` _asbp_bike_project_game_mode_base)
  (`KismetSystemLibrary.Delay` 2.0)
  (`self.K2_DestroyActor`)
  (`self.Destroy Building Instances`))

(fn `Destroy Building Instances`
  (`/Game/Blueprints/Art/BP_Buildings.Destroy Buildings` (`self.Building Reference`)))

(fn `GetAttachTransform`
  (returns (AttachTransform :type "Transform Structure"))
  (return (`SceneComponent.K2_GetComponentToWorld` (`self.AttachPoint`))))

(fn `SetSpawnArray`
  (set `self.SpawnPoints` (`|MakeArray` (`SceneComponent.GetRelativeTransform` (`self.ObstacleSpawnR`)) (`SceneComponent.GetRelativeTransform` (`self.ObstacleSpawnC`)) (`SceneComponent.GetRelativeTransform` (`self.ObstacleSpawnL`)))))

(fn `SpawnObstacleChecker`
  (for (_array_element _array_index) (`self.SpawnPoints`)
    (bind _returnvalue (`AddComponent|NODE_AddChildActorComponent-0` :`RelativeTransform` _array_element))
    (bind _asbp_obstacle_checker (cast `/Game/Blueprints/BP_ObstacleChecker` (`ChildActorComponent.ChildActor` _returnvalue)))
    (set `/Game/Blueprints/BP_ObstacleChecker.Lane` _array_index _asbp_obstacle_checker)))

(fn `UserConstructionScript`
  (`self.SetSpawnArray`)
  (bind _returnvalue (`GameplayStatics.GetActorOfClass` "/Game/Blueprints/Art/BP_LevelDatabaseActor.BP_LevelDatabaseActor_C"))
  (bind _tiles (`/Game/Blueprints/Art/BP_LevelDatabaseActor.Tiles` _returnvalue))
  (`ChildActorComponent.SetChildActorClass` (`self.ChildActor`) (`|GetArrayItem` _tiles (`KismetMathLibrary.RandomIntegerInRange` 0 (- (`KismetArrayLibrary.Array_Length` _tiles) 1))))
  (switch `/Game/Blueprints/ObstacleType` (`self.Obstacle Spawn`)
    (:`NewEnumerator1`
      (`self.SpawnObstacleChecker`))))