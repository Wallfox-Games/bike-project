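; AI controller for peep pawns that starts their behavior tree when the player is nearby.
; It stores the possessed pawn, then each Tick compares its distance to player pawn 0 and calls RunBehaviorTree with PeepsBT while within range.
; Nothing stops the tree out of range, despite a comment about deleting it.
; Unconnected leftovers pick a random offset destination and run a walking tree at a wider range.
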(event `self.ReceivePossess`
  (params (PossessedPawn :type "Pawn Object Reference"))
  (set `self.Possessed Pawn` PossessedPawn))

(event `self.ReceiveTick`
  (params (DeltaSeconds :type "Float (single-precision)"))
  ;[1 1 1] If player is within range
  (if (<= (`KismetMathLibrary.Vector_Distance` (`self.K2_GetActorLocation` (`self.Possessed Pawn`)) (`self.K2_GetActorLocation` (`GameplayStatics.GetPlayerPawn` 0))) 2000.0)
    ;[1 1 1] Run behaviour tree and delete once out of view
    (`self.RunBehaviorTree` "/Game/Blueprints/Peeps/PeepsBT.PeepsBT")))

(fn `UserConstructionScript`)