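; Behavior tree task that gives a BP_Peeps4 pawn its walking destination.
; It casts the controlled pawn, copies its WalkingDes into a blackboard vector key and finishes successfully.
; If the cast fails, execution stops without calling FinishExecute.
; An unconnected branch that picks a random point 2000 units either way along X from the current location never runs.
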(event `self.ReceiveExecuteAI`
  (params (OwnerController :type "AIController Object Reference") (ControlledPawn :type "Pawn Object Reference"))
  (bind _asbp_peeps_4 (cast `/Game/Blueprints/Peeps/BP_Peeps4` ControlledPawn))
  (bind _output_get (set `self.Destination` (`/Game/Blueprints/Peeps/BP_Peeps4.WalkingDes` _asbp_peeps_4)))
  (`BTFunctionLibrary.SetBlackboardValueAsVector` (`self.Key`) _output_get)
  (`self.FinishExecute` true))