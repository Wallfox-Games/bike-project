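; Behavior tree task for peeps that picks a new destination relative to the controlled pawn's current location.
; On execute, it randomly chooses one of four fixed offsets: a large step along positive or negative Y, with or without a small forward shift in X, keeping Z.
; It writes the point to a Blackboard vector key and finishes successfully, without any navmesh or reachability check.
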(event `self.ReceiveExecuteAI`
  (params (OwnerController :type "AIController Object Reference") (ControlledPawn :type "Pawn Object Reference"))
  (bind _z (`self.Z`))
  (bind _returnvalue (- (`self.X`) 0.0))
  (bind _returnvalue_2 (+ (`self.X`) 150.0))
  (set `self.X` (.x (`Actor.K2_GetActorLocation` ControlledPawn)))
  (set `self.Y value` (.y (`Actor.K2_GetActorLocation` ControlledPawn)))
  (set `self.Z` (.z (`Actor.K2_GetActorLocation` ControlledPawn)))
  (bind _output_get (set `self.DestinationDirection` (`KismetMathLibrary.RandomIntegerInRange` 0 3)))
  (switch `int` _output_get
    (:`0`
      (bind _output_get_2 (set `self.Y value` (+ (`self.Y value`) 630.0)))
      (set `self.Destination` (`KismetMathLibrary.MakeVector` _returnvalue_2 _output_get_2 _z)))
    (:`1`
      (bind _output_get_3 (set `self.Y value` (+ (`self.Y value`) 630.0)))
      (set `self.Destination` (`KismetMathLibrary.MakeVector` _returnvalue _output_get_3 _z)))
    (:`2`
      (bind _output_get_4 (set `self.Y value` (- (`self.Y value`) 630.0)))
      (set `self.Destination` (`KismetMathLibrary.MakeVector` _returnvalue_2 _output_get_4 _z)))
    (:`3`
      (bind _output_get_5 (set `self.Y value` (- (`self.Y value`) 630.0)))
      (set `self.Destination` (`KismetMathLibrary.MakeVector` _returnvalue _output_get_5 _z))))
  (`BTFunctionLibrary.SetBlackboardValueAsVector` (`self.Key`) (`self.Destination`))
  (`self.FinishExecute` true))