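; BP_Peeps3 is an AI-moved pawn that walks to a fixed spot offset along negative Y from its start when the player comes near.
; Tick checks player distance and issues AIMoveTo every frame in range, printing a debug message and retrying on failure.
; BeginPlay caches that destination and a random upward launch vector.
; The capsule hit event is empty, leaving the player-triggered impulse using that vector disconnected.
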(event `self.ReceiveBeginPlay`
  (set `self.LaunchDirection` (`KismetMathLibrary.MakeVector` (* 5000 (`KismetMathLibrary.RandomFloat`)) (* 5000 (`KismetMathLibrary.RandomFloatInRange` -1.0 1.0)) 5000.0))
  (set `self.Destination` (`KismetMathLibrary.MakeVector` (.x (`self.K2_GetActorLocation`)) (- (.y (`self.K2_GetActorLocation`)) 340.0) (.z (`self.K2_GetActorLocation`)))))

(event `self.ReceiveTick`
  (params (DeltaSeconds :type "Float (single-precision)"))
  (if (<= (`KismetMathLibrary.Vector_Distance` (`self.K2_GetActorLocation`) (`self.K2_GetActorLocation` (`GameplayStatics.GetPlayerPawn` 0))) 1000.0)
    (`|AIMoveTo` self (`self.Destination`) null 1.0 :!label _label
      (:`OnFail`
        (`KismetSystemLibrary.PrintString` "bad")
        (goto _label)))))

(event `self.CapsuleComponent.OnComponentHit`
  (params (HitComponent :type "PrimitiveComponent Object Reference") (OtherActor :type "Actor Object Reference") (OtherComp :type "PrimitiveComponent Object Reference") (NormalImpulse :type "Vector Structure") (Hit :type "HitResult Structure (by ref)")))

(fn `UserConstructionScript`)