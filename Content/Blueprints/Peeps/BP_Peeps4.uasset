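; BP_Peeps4 is a pedestrian character that reacts to the player's proximity and can be knocked into the air.
; BeginPlay picks a random diagonal destination and walk speed, but the AI move and stuck-nudge logic are disconnected.
; Tick raises walk speed near the player; very close contact triggers an interpolated upward launch with physics toggling.
; The proximity path also leads to delayed destruction, even without a hit.
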(event `self.ReceiveBeginPlay`
  (bind _z (`self.Z`))
  (bind _returnvalue (- (`self.X`) 600.0))
  (bind _returnvalue_2 (+ (`self.X`) 600.0))
  (set `self.Beenhit` false)
  (set `self.X` (.x (`self.K2_GetActorLocation` self)))
  (set `self.Y value` (.y (`self.K2_GetActorLocation` self)))
  (set `self.Z` (.z (`self.K2_GetActorLocation` self)))
  (bind _output_get (set `self.DestinationDirection` (`KismetMathLibrary.RandomIntegerInRange` 0 3)))
  (switch `int` _output_get
    (:`0`
      (bind _output_get_2 (set `self.Y value` (+ (`self.Y value`) 630.0)))
      (set `self.Destination` (`KismetMathLibrary.MakeVector` _returnvalue_2 _output_get_2 _z)))
    (:`1`
      (bind _output_get_3 (set `self.Y value` (+ (`self.Y value`) 630.0)))
      (set `self.Destination` (`KismetMathLibrary.MakeVector` _returnvalue _output_get_3 _z)))
    (:`2`
      (bind _output_get_4 (set `self.Y value` (- (`self.Y value`) 630.0)))
      (set `self.Destination` (`KismetMathLibrary.MakeVector` _returnvalue_2 _output_get_4 _z)))
    (:`3`
      (bind _output_get_5 (set `self.Y value` (- (`self.Y value`) 630.0)))
      (set `self.Destination` (`KismetMathLibrary.MakeVector` _returnvalue _output_get_5 _z))))
  (set `CharacterMovementComponent.MaxWalkSpeed` 200.0 (`self.CharacterMovement`)))

(event `self.ReceiveTick`
  (params (DeltaSeconds :type "Float (single-precision)"))
  (bind _returnvalue (`self.K2_GetActorLocation` self))
  (bind _returnvalue_2 (`KismetMathLibrary.Vector_Distance` _returnvalue (`self.K2_GetActorLocation` (`GameplayStatics.GetPlayerPawn` 0))))
  (if (`self.Beenhit`)
    (`self.K2_SetActorLocation` self (`KismetMathLibrary.VInterpTo` (`self.K2_GetActorLocation` self) (`self.Flight path`) DeltaSeconds 2.0) false false)
    (`KismetSystemLibrary.Delay` 2.0)
    (`PrimitiveComponent.SetSimulatePhysics` (`self.CapsuleComponent`) false)
    (if (== (stale _output_get) _returnvalue) :!label _label
      (`/Engine/EditorBlueprintResources/StandardMacros.IncrementInt` (`self.Stationary counter`)
        (:`  `
          _)))
    (if (== (`self.Stationary counter`) 5)
      _
      (else
        _))
    (if (<= (`KismetMathLibrary.Vector_Distance` (`self.K2_GetActorLocation` self) (`self.K2_GetActorLocation` (`GameplayStatics.GetPlayerPawn` 0))) 75.0)
      (set `self.Beenhit` true)
      (set `self.Flight path` (`KismetMathLibrary.MakeVector` (.x (`self.K2_GetActorLocation`)) (.y (`self.K2_GetActorLocation`)) (+ (.z (`self.K2_GetActorLocation`)) 500.0)))
      (`PrimitiveComponent.SetSimulatePhysics` (`self.CapsuleComponent`) true))
    (`KismetSystemLibrary.Delay` 4.0)
    (`self.K2_DestroyActor`)
    (else
      (bind _output_get (set `self.PrePosition` _returnvalue))
      (if (<= _returnvalue_2 2000.0)
        (if (<= _returnvalue_2 500.0)
          (set `CharacterMovementComponent.MaxWalkSpeed` 400.0 (`self.CharacterMovement`))
          (goto _label)
          (else
            (goto _label)))))))

(fn `UserConstructionScript`)