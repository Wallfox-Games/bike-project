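; BP_Peeps2 is a peep actor that gets knocked into the air when the player pawn hits it.
; BeginPlay rolls a random launch vector with fixed upward strength, which Hit applies as an impulse to the root component.
; Tick issues AIMoveTo with no inputs set and prints a dinosaur panic message.
; A player-distance check exists but is unconnected.
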(event `self.ReceiveBeginPlay`
  (set `self.Launch direction` (`KismetMathLibrary.MakeVector` (* 5000 (`KismetMathLibrary.RandomFloat`)) (* 5000 (`KismetMathLibrary.RandomFloatInRange` -1.0 1.0)) 5000.0)))

(event `self.ReceiveActorBeginOverlap`
  (params (OtherActor :type "Actor Object Reference")))

(event `self.ReceiveTick`
  (params (DeltaSeconds :type "Float (single-precision)"))
  (`|AIMoveTo` null (0.0 0.0 0.0) null
    (:`then`
      (`KismetSystemLibrary.PrintString` "RUN ITS A DINOSAUR"))))

(event `self.ReceiveHit`
  (params (MyComp :type "PrimitiveComponent Object Reference") (Other :type "Actor Object Reference") (OtherComp :type "PrimitiveComponent Object Reference") (bSelfMoved :type Boolean) (HitLocation :type "Vector Structure") (HitNormal :type "Vector Structure") (NormalImpulse :type "Vector Structure") (Hit :type "HitResult Structure (by ref)"))
  (if (== Other (`GameplayStatics.GetPlayerPawn` 0))
    (`PrimitiveComponent.AddImpulse` (`self.Root Component`) (`self.Launch direction`) "None" false)))

(fn `UserConstructionScript`)