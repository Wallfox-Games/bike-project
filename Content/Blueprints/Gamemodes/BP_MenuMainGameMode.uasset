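; Main menu game mode that lays out a short piece of floor track when play begins in a bike game.
; It sets a fixed, angled spawn transform and zeroes the tile count, then calls AddFloorTile for two straight tiles and a 90-degree bend.
; It then sets the mobile state on the BikeGameInstance; Tick is disabled.
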(event `self.ReceiveBeginPlay`
  (`parent.ReceiveBeginPlay`)
  (set `self.NextSpawnPoint` (`KismetMathLibrary.MakeTransform` (-30.0 -300.0 -50.0) (struct :`Yaw` 45.0)))
  (set `self.Current Tile Count` 0)
  (`self.Add Floor Tile` "NewEnumerator0")
  (`self.Add Floor Tile` "NewEnumerator0")
  (`self.Add Floor Tile` "NewEnumerator0" true 90.0)
  (bind _asbike_game_instance (cast `BikeGameInstance` (`GameplayStatics.GetGameInstance`)))
  (`BikeGameInstance.SetMobileState` _asbike_game_instance 1))

(fn `UserConstructionScript`
  (`parent.UserConstructionScript`))