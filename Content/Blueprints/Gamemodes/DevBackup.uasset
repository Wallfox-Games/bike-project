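; DevBackup, in the Gamemodes folder, builds a road tile by tile, chaining each piece from the previous one's attach transform.
; AddFloorTile spawns either a straight floor tile or a randomly angled left or right bend, with bends growing likelier as straight tiles accumulate.
; Level_Tutorial always gets straight tiles.
; Straight tiles also have the level's BP_Buildings actor place buildings, using the running tile count.
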(event `self.ReceiveBeginPlay`
  (bind _returnvalue (`GameplayStatics.GetActorOfClass` "/Game/Blueprints/Art/BP_Buildings.BP_Buildings_C"))
  (set `self.Building Reference` _returnvalue))

(event `self.ReceiveTick`
  (params (DeltaSeconds :type "Float (single-precision)")))

(fn `Add Floor Tile`
  (params (Obstacle :type "/Game/Blueprints/Tiles/ObstacleType Enum" :default "NewEnumerator0"))
  (bind _nextspawnpoint (`self.NextSpawnPoint`))
  (bind _returnvalue (* (`self.i`) 10.0))
  (bind _returnvalue_2 (`KismetMathLibrary.MakeTransform` (.location _nextspawnpoint) (`KismetMathLibrary.MakeRotator` (.roll (.rotation _nextspawnpoint)) (.pitch (.rotation _nextspawnpoint)) (- (.yaw (.rotation _nextspawnpoint)) 90.0)) (.scale _nextspawnpoint)))
  (bind _returnvalue_3 (`GameplayStatics.GetCurrentLevelName` true))
  (set `self.i` 0)
  (if (`KismetStringLibrary.EqualEqual_StrStr` _returnvalue_3 "Level_Tutorial")
    (bind _returnvalue_4 (`|SpawnActorFromClass` "/Game/Blueprints/Tiles/BP_FloorTile.BP_FloorTile_C" _nextspawnpoint "Undefined" "OverrideRootScale" null Obstacle null :!label _label))
    (`self.Spawn Buildings` _nextspawnpoint)
    (bind _attachtransform (`/Game/Blueprints/Tiles/BP_FloorTile.GetAttachTransform` _returnvalue_4))
    (set `self.NextSpawnPoint` _attachtransform)
    (`/Engine/EditorBlueprintResources/StandardMacros.IncrementInt` (`self.Tiles Since Last Bend`)
      (:`  `
        _))
    (elif (== (`KismetMathLibrary.RandomIntegerInRange` 0 (- 15 (`self.Tiles Since Last Bend`))) 0)
      (while (== (`self.i`) 0)
        (set `self.i` (`KismetMathLibrary.RandomIntegerInRange` -2 2)))
      (bind _returnvalue_5 (`|SpawnActorFromClass` "/Game/Blueprints/Art/BP_BendRoad.BP_BendRoad_C" _returnvalue_2 "Undefined" "OverrideRootScale" null _returnvalue _returnvalue_2 null))
      (bind _attach_transform (`/Game/Blueprints/Art/BP_BendRoad.Get Attach Transform` _returnvalue_5))
      (set `self.NextSpawnPoint` (`KismetMathLibrary.MakeTransform` (.location _attach_transform) (`KismetMathLibrary.MakeRotator` 0.0 0.0 (+ (.yaw (.rotation (`self.NextSpawnPoint`))) _returnvalue))))
      (set `self.Tiles Since Last Bend` 0)
      (else
        (goto _label))))
  (`self.Increment Tile Count`))

(fn `Get Progressed`
  (returns (Progressed :type "Float (double-precision)"))
  (return (`self.Progressed`)))

(fn `Increment Tile Count`
  (set `self.Current Tile Count` (+ (`self.Current Tile Count`) 1)))

(fn `Next Floor Tile`)

(fn `Spawn Buildings`
  (params (`Spawn Transform` :type "Transform Structure"))
  (`/Game/Blueprints/Art/BP_Buildings.Place Buildings` (`self.Building Reference`) `Spawn Transform` (`self.Current Tile Count`)))

(fn `UserConstructionScript`)