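; Debug game mode for a lane-based bike game, letting a tester control floor tile spawning by keyboard.
; While no boss is active, Tick polls keys to queue blank, good, bad or bend tiles, spawn a boss or raise health, and prints the queue and upcoming obstacles.
; NextFloorTile consumes that queue, randomizing bend direction and angle.
; Tick also removes defeated bosses after a delay and fades to the main menu at zero health.
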(event `self.ReceiveBeginPlay`
  (`parent.ReceiveBeginPlay`)
  (for _ (range 10)
    (`self.Next Floor Tile`))
  (`GameplayStatics.PlaySound2D` "/Game/SoundFiles/SoundCues/LevelMusicSoundCue.LevelMusicSoundCue" 1.0 1.0 0.0 null null)
  (bind _asbike_game_instance (cast `BikeGameInstance` (`GameplayStatics.GetGameInstance`)))
  (`BikeGameInstance.SetMobileState` _asbike_game_instance 2))

(event `self.ReceiveTick`
  (params (DeltaSeconds :type "Float (single-precision)"))
  (bind _bossreference (`self.BossReference`))
  (bind _obstaclearraycontents (`self.ObstacleArrayContents`))
  (`parent.ReceiveTick` DeltaSeconds)
  (bind _asbp_bike_player_controller (cast `/Game/Blueprints/Player/BP_BikePlayerController` (`GameplayStatics.GetPlayerController` 0)))
  (if (!= (`BikeProjectPlayerController.GetPlayerHealth` _asbp_bike_player_controller) 0)
    (if (== _bossreference null)
      (`self.Add To Obstacle Array`)
      (`self.Get Next Tile Info` DeltaSeconds)
      (for _array_element (`self.ObstacleSpawnArray`)
        (switch `int` _array_element
          (:`Default`
            (set `self.ObstacleArrayContents` (`KismetStringLibrary.Concat_StrStr` _obstaclearraycontents "Blank, ") :!label _label))
          (:`0`
            (goto _label))
          (:`1`
            (set `self.ObstacleArrayContents` (`KismetStringLibrary.Concat_StrStr` _obstaclearraycontents "Good, ")))
          (:`2`
            (set `self.ObstacleArrayContents` (`KismetStringLibrary.Concat_StrStr` _obstaclearraycontents "Bad, ")))
          (:`3`
            (set `self.ObstacleArrayContents` (`KismetStringLibrary.Concat_StrStr` _obstaclearraycontents "Bend, ")))))
      (`KismetSystemLibrary.PrintString` _obstaclearraycontents true true (struct :`G` 0.66 :`B` 1.0 :`A` 1.0) DeltaSeconds)
      (set `self.ObstacleArrayContents` "")
      (else
        (switch `EBossState` (`BikeBoss.GetBossEnum` _bossreference)
          (:`BSE_Defeated`
            (`self.Destroy Boss` DeltaSeconds)))))
    (else
      (`BikeProjectPlayerController.SetMoveUIBlocked` _asbp_bike_player_controller true)
      (bind _level_widget_reference (`/Game/Blueprints/Player/BP_BikePlayerController.Level Widget Reference` _asbp_bike_player_controller))
      (bind _fade (`/Game/UserInterface/HUD/HUDLevel.Fade` _level_widget_reference))
      (if (`UserWidget.IsAnimationPlaying` _level_widget_reference _fade)
        (`KismetSystemLibrary.Delay` (`WidgetAnimation.GetEndTime` _fade))
        (`GameplayStatics.OpenLevel` "Menu_Main")
        (else
          (`/Game/UserInterface/HUD/HUDLevel.Start Fade` _level_widget_reference false))))))

(fn `Add To Obstacle Array`
  (bind _returnvalue (`GameplayStatics.GetPlayerController` 0))
  (bind _obstaclespawnarray (`self.ObstacleSpawnArray`))
  (bind _returnvalue_2 (`KismetArrayLibrary.Array_Length` _obstaclespawnarray))
  (if (`PlayerController.WasInputKeyJustPressed` _returnvalue "B")
    (`KismetArrayLibrary.Array_Insert` _obstaclespawnarray 0 _returnvalue_2)
    (elif (`PlayerController.WasInputKeyJustPressed` _returnvalue "N")
      (`KismetArrayLibrary.Array_Insert` _obstaclespawnarray 1 _returnvalue_2)
      (elif (`PlayerController.WasInputKeyJustPressed` _returnvalue "M")
        (`KismetArrayLibrary.Array_Insert` _obstaclespawnarray 2 _returnvalue_2)
        (elif (`PlayerController.WasInputKeyJustPressed` _returnvalue "Comma")
          (`KismetArrayLibrary.Array_Insert` _obstaclespawnarray 3 _returnvalue_2)
          (elif (`PlayerController.WasInputKeyJustPressed` _returnvalue "SpaceBar")
            (`self.Spawn Boss`)
            (elif (`PlayerController.WasInputKeyJustPressed` _returnvalue "H")
              (bind _asbp_bike_player_controller (cast `/Game/Blueprints/Player/BP_BikePlayerController` _returnvalue))
              (`BikeProjectPlayerController.IncPlayerHealth` _asbp_bike_player_controller true))))))))

(fn `Destroy Boss`
  (params (`Delta Time` :type "Float (double-precision)"))
  (bind _bossdespawntimer (`self.BossDespawnTimer`))
  (if (>= _bossdespawntimer 1.0)
    (`self.K2_DestroyActor` (`self.BossReference`))
    (set `self.BossReference` null)
    (else
      (set `self.BossDespawnTimer` (+ _bossdespawntimer `Delta Time`)))))

(fn `Get Next Tile Info`
  (params (DeltaTime :type "Float (double-precision)"))
  (set `self.Second Tile Info` false)
  (for _array_element (`self.Tile Info Array`)
    (bind (_floortilereference _bendtilereference _obstacletype _obstaclelanes) (break `/Game/Blueprints/Tiles/ST_TileInfo` _array_element))
    (if (`|EnumInequality` _obstacletype "NewEnumerator0")
      (if (`self.Second Tile Info`)
        (break)
        (else
          (set `self.Second Tile Info` true)
          (`KismetSystemLibrary.PrintText` (`|FormatText` "Obstacle {obstacle} in Lanes {a} {b} {c}" (`KismetMathLibrary.Conv_ByteToInt` _obstacletype) (`|GetArrayItem` _obstaclelanes) (`|GetArrayItem` _obstaclelanes 1) (`|GetArrayItem` _obstaclelanes 2)) true true (struct :`G` 0.66 :`B` 1.0 :`A` 1.0) DeltaTime :!label _label)))))
  (goto _label))

(fn `Next Floor Tile`
  (bind _obstaclespawnarray (`self.ObstacleSpawnArray`))
  (bind _returnvalue (+ (* (`KismetMathLibrary.RandomFloat`) 30.0) 10.0))
  (`parent.Next Floor Tile`)
  (if (or (== (`self.BossReference`) null) (== (`KismetArrayLibrary.Array_Length` _obstaclespawnarray) 0))
    (switch `int` (`|GetArrayItem` _obstaclespawnarray)
      (:`Default`
        (`self.Add Floor Tile` "NewEnumerator0" :!label _label)
        (`KismetArrayLibrary.Array_Remove` _obstaclespawnarray))
      (:`0`
        (goto _label))
      (:`1`
        (`self.Add Floor Tile` "NewEnumerator1")
        (`KismetArrayLibrary.Array_Remove` _obstaclespawnarray))
      (:`2`
        (`self.Add Floor Tile` "NewEnumerator2")
        (`KismetArrayLibrary.Array_Remove` _obstaclespawnarray))
      (:`3`
        (if (`KismetMathLibrary.RandomBool`)
          (`self.Add Floor Tile` "NewEnumerator0" true (* _returnvalue -1.0))
          (`KismetArrayLibrary.Array_Remove` _obstaclespawnarray)
          (else
            (`self.Add Floor Tile` "NewEnumerator0" true _returnvalue)
            (`KismetArrayLibrary.Array_Remove` _obstaclespawnarray)))))
    (else
      (goto _label))))

(fn `Reset Tiles`
  (bind _outactors (`GameplayStatics.GetAllActorsOfClass` "/Game/Blueprints/Tiles/BP_FloorTile.BP_FloorTile_C"))
  (for _array_element _outactors
    (`/Game/Blueprints/Tiles/BP_FloorTile.Destroy Self` _array_element))
  (bind _outactors_2 (`GameplayStatics.GetAllActorsOfClass` "/Game/Blueprints/Art/BP_BendRoad.BP_BendRoad_C"))
  (for _array_element_2 _outactors_2
    (`self.K2_DestroyActor` _array_element_2))
  (for _ (range 10)
    (`self.Next Floor Tile`)))

(fn `Spawn Boss`
  (bind _returnvalue (`|SpawnActorFromClass` "/Game/Blueprints/Boss/BP_BikeBoss.BP_BikeBoss_C" (`KismetMathLibrary.MakeTransform` (0.0 0.0 0.0)) "AlwaysSpawn" "OverrideRootScale" null null))
  (bind _output_get (set `self.BossReference` _returnvalue))
  (bind _asbp_player_character (cast `/Game/Blueprints/Player/BP_PlayerCharacter` (`GameplayStatics.GetPlayerPawn` 0)))
  (`BikeBoss.InitValues` _output_get _asbp_player_character 3 20.0 0.7 0.0)
  (set `self.BossDespawnTimer` 0.0))

(fn `UserConstructionScript`
  (`parent.UserConstructionScript`))