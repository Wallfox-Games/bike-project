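; Endless-mode game mode for the bike game, running procedurally generated track through repeating boss stages.
; NextFloorTile randomly adds bends or obstacle tiles, weighted by difficulty and player health, leaving stage starts and boss approaches plain.
; Tick flashes a warning before the boss tile, spawns a difficulty-scaled boss, then on its defeat advances the stage and shows results.
; During results the bike slows, and the level ends once power drops low.
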(event `self.ReceiveBeginPlay`
  (`parent.ReceiveBeginPlay`)
  (for _ (range 10)
    (`self.Next Floor Tile`))
  (`GameplayStatics.PlaySound2D` "/Game/SoundFiles/SoundCues/LevelMusicSoundCue.LevelMusicSoundCue" 1.0 1.0 0.0 null null)
  (bind _asbike_game_instance (cast `BikeGameInstance` (`GameplayStatics.GetGameInstance`)))
  (`BikeGameInstance.SetMobileState` _asbike_game_instance 2))

(event `self.ReceiveTick`
  (params (DeltaSeconds :type "Float (single-precision)"))
  (bind _bossreference (`self.BossReference`))
  (bind _current_tile_count (`self.Current Tile Count`))
  (`parent.ReceiveTick` DeltaSeconds)
  (bind _asbp_bike_player_controller (cast `/Game/Blueprints/Player/BP_BikePlayerController` (`GameplayStatics.GetPlayerController` 0)))
  (bind _level_widget_reference (`/Game/Blueprints/Player/BP_BikePlayerController.Level Widget Reference` _asbp_bike_player_controller))
  (if (`/Game/UserInterface/HUD/HUDLevel.InResults` _level_widget_reference)
    _
    (elif (!= (`BikeProjectPlayerController.GetPlayerHealth` _asbp_bike_player_controller) 0)
      (`KismetSystemLibrary.PrintString` (`KismetTextLibrary.Conv_TextToString` (`|FormatText` "Tile Count: {0}" _current_tile_count)) true true (struct :`G` 0.66 :`B` 1.0 :`A` 1.0) DeltaSeconds)
      (if (== _bossreference null)
        (if (== _current_tile_count (- (`self.Boss Spawn Tile`) 10))
          (`/Game/UserInterface/HUD/HUDLevel.Set Text Flash` _level_widget_reference true)
          (elif (== (`self.Current Tile Count`) (`self.Boss Spawn Tile`))
            (`self.Spawn Difficulty Boss` DeltaSeconds)
            (`/Game/UserInterface/HUD/HUDLevel.Set Text Flash` _level_widget_reference false)))
        (else
          (switch `EBossState` (`BikeBoss.GetBossEnum` _bossreference)
            (:`BSE_Defeated`
              (bind _boss_destroyed (`self.Destroy Boss` DeltaSeconds))
              (if _boss_destroyed
                (`self.Next Stage`)
                (`/Game/UserInterface/HUD/HUDLevel.Show Results` _level_widget_reference false))))))
      (else
        (`BikeProjectPlayerController.SetMoveEnum` _asbp_bike_player_controller "PME_SlowDown" DeltaSeconds)
        (if (<= (`BikeProjectPlayerController.GetPowerLevel` _asbp_bike_player_controller) 0.5)
          (`/Game/UserInterface/HUD/HUDLevel.End Level` _level_widget_reference))))))

(fn `Next Floor Tile`
  (bind _boss_spawn_tile (`self.Boss Spawn Tile`))
  (bind _difficulty (`self.Difficulty`))
  (bind _current_tile_count (`self.Current Tile Count`))
  (bind _returnvalue (+ (* (`KismetMathLibrary.RandomFloat`) 30.0) 10.0))
  (`parent.Next Floor Tile`)
  (set `self.Progressed` (/ (`KismetMathLibrary.Conv_IntToDouble` _current_tile_count) (`KismetMathLibrary.Conv_IntToDouble` _boss_spawn_tile)))
  (if (and (== (`self.BossReference`) null) (>= (- _boss_spawn_tile 11) _current_tile_count) (> _current_tile_count 5))
    (if (== (`KismetMathLibrary.RandomIntegerInRange` 0 (- 15 (`self.Tiles Since Last Bend`))) 0)
      (if (`KismetMathLibrary.RandomBool`)
        (`self.Add Floor Tile` "NewEnumerator0" true (* _returnvalue -1.0))
        (else
          (`self.Add Floor Tile` "NewEnumerator0" true _returnvalue)))
      (elif (== (mod _current_tile_count (`KismetMathLibrary.RandomIntegerInRange` 2 (`KismetMathLibrary.Clamp` (- 4 _difficulty) 2 4))) 1)
        (if (>= _difficulty (`KismetMathLibrary.RandomIntegerInRange` 0 (+ _difficulty 3)))
          (`self.Add Floor Tile` "NewEnumerator1")
          (else
            (bind _asbp_bike_player_controller (cast `/Game/Blueprints/Player/BP_BikePlayerController` (`GameplayStatics.GetPlayerController` 0)))
            (if (>= (`KismetMathLibrary.RandomIntegerInRange` -5 8) (`BikeProjectPlayerController.GetPlayerHealth` _asbp_bike_player_controller))
              (`self.Add Floor Tile` "NewEnumerator4")
              (else
                (`self.Add Floor Tile` "NewEnumerator2")))))
        (else
          (`self.Add Floor Tile` "NewEnumerator0" :!label _label))))
    (else
      (goto _label))))

(fn `Spawn Difficulty Boss`
  (params (`Delta Time` :type "Float (double-precision)"))
  (switch `int` (`self.Difficulty`)
    (:`0`
      (`self.Spawn Boss` 2 20.0 0.7 `Delta Time`))
    (:`1`
      (`self.Spawn Boss` 2 20.0 0.8 `Delta Time`))
    (:`2`
      (`self.Spawn Boss` 3 20.0 0.8 `Delta Time`))
    (:`3`
      (`self.Spawn Boss` 3 25.0 0.8 `Delta Time`))
    (:`4`
      (`self.Spawn Boss` 3 25.0 0.85 `Delta Time`))))

(fn `UserConstructionScript`
  (`parent.UserConstructionScript`))