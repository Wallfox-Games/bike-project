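; Tutorial game mode for a bike runner that teaches speed, lane changes, pickups, hazards and a boss fight in stages.
; Tick advances TutorialState by floor tile count, initially blocking lane changes, then by the spawned boss's state.
; The NextFloorTile override uses that state to place stage-specific obstacles periodically on straight tiles.
; Health is topped up before and during the weakened boss fight; after victory the bike slows until results show.
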(event `self.ReceiveBeginPlay`
  (`parent.ReceiveBeginPlay`)
  (for _ (range 6)
    (`self.Next Floor Tile`))
  (bind _asbike_game_instance (cast `BikeGameInstance` (`GameplayStatics.GetGameInstance`)))
  (`BikeGameInstance.SetMobileState` _asbike_game_instance 2)
  (bind _returnvalue (`|CreateWidget` "/Game/UserInterface/HUD/HUDTutorial.HUDTutorial_C" (`GameplayStatics.GetPlayerController` 0)))
  (`UserWidget.AddToViewport` _returnvalue 0))

(event `self.ReceiveTick`
  (params (DeltaSeconds :type "Float (single-precision)"))
  (bind _returnvalue (`GameplayStatics.GetPlayerPawn` 0))
  (bind _returnvalue_2 (`GameplayStatics.GetPlayerController` 0))
  (bind _bossreference (`self.BossReference`))
  (bind _current_tile_count (`self.Current Tile Count`))
  (`parent.ReceiveTick` DeltaSeconds)
  (if (<= _current_tile_count 15)
    (set `self.TutorialState` "NewEnumerator0")
    (bind _asbp_player_character (cast `/Game/Blueprints/Player/BP_PlayerCharacter` _returnvalue))
    (`BikeCharacter.SetLaneBlocked` _asbp_player_character true)
    (`BikeCharacter.SetMaxPower` _asbp_player_character 12.0)
    (elif (<= _current_tile_count 30)
      (set `self.TutorialState` "NewEnumerator10")
      (elif (<= _current_tile_count 60)
        (set `self.TutorialState` "NewEnumerator1")
        (bind _asbp_player_character_2 (cast `/Game/Blueprints/Player/BP_PlayerCharacter` _returnvalue))
        (`BikeCharacter.SetLaneBlocked` _asbp_player_character_2 false)
        (elif (<= _current_tile_count 80)
          (set `self.TutorialState` "NewEnumerator2")
          (elif (<= _current_tile_count 100)
            (set `self.TutorialState` "NewEnumerator6")
            (elif (<= _current_tile_count 120)
              (set `self.TutorialState` "NewEnumerator4")
              (elif (<= _current_tile_count 135)
                (set `self.TutorialState` "NewEnumerator9")
                (bind _asbp_bike_player_controller (cast `/Game/Blueprints/Player/BP_BikePlayerController` _returnvalue_2))
                (if (!= (`BikeProjectPlayerController.GetPlayerHealth` _asbp_bike_player_controller) 8)
                  (`BikeProjectPlayerController.IncPlayerHealth` _asbp_bike_player_controller true))
                (elif (`|EnumEquality` (`self.TutorialState`) "NewEnumerator8")
                  (bind _asbp_bike_player_controller_2 (cast `/Game/Blueprints/Player/BP_BikePlayerController` _returnvalue_2))
                  (if (not (`/Game/UserInterface/HUD/HUDLevel.InResults` (`/Game/Blueprints/Player/BP_BikePlayerController.Level Widget Reference` _asbp_bike_player_controller_2)))
                    (switch `EPlayerMove` (`BikeProjectPlayerController.GetMoveEnum` _asbp_bike_player_controller_2)
                      (:`PME_Normal`
                        (`BikeProjectPlayerController.SetMoveEnum` _asbp_bike_player_controller_2 "PME_SlowDown" DeltaSeconds :!label _label))
                      (:`PME_BossCharge`
                        (goto _label))
                      (:`PME_BossDodge`
                        (goto _label))
                      (:`PME_BossAttack`
                        (goto _label))
                      (:`PME_BossCooldown`
                        (goto _label))
                      (:`PME_SlowDown`
                        _))
                    (if (<= (`BikeProjectPlayerController.GetPowerLevel` _asbp_bike_player_controller_2) 0.5)
                      (`self.Show Results`)))
                  (elif (== _bossreference null)
                    (`self.Spawn Boss` 1 30.0 0.5)
                    (else
                      (switch `EBossState` (`BikeBoss.GetBossEnum` _bossreference)
                        (:`BSE_Attacking`
                          (set `self.TutorialState` "NewEnumerator7"))
                        (:`BSE_Despawning`
                          (bind _asbp_bike_player_controller_3 (cast `/Game/Blueprints/Player/BP_BikePlayerController` _returnvalue_2))
                          (if (== (`BikeProjectPlayerController.GetPlayerHealth` _asbp_bike_player_controller_3) 1)
                            (`BikeProjectPlayerController.IncPlayerHealth` _asbp_bike_player_controller_3 true)))
                        (:`BSE_Reloading`
                          (set `self.TutorialState` "NewEnumerator11"))
                        (:`BSE_Defeated`
                          (set `self.TutorialState` "NewEnumerator8")
                          (bind _boss_destroyed (`self.Destroy Boss` DeltaSeconds))
                          (if _boss_destroyed
                            (set `self.TutorialState` "NewEnumerator8")))))))))))))))

(fn `Next Floor Tile`
  (bind _returnvalue (== (mod (`self.Current Tile Count`) 4) 0))
  (`parent.Next Floor Tile`)
  (set `self.Progressed` (/ (`KismetMathLibrary.Conv_IntToDouble` (`self.Current Tile Count`)) (`KismetMathLibrary.Conv_IntToDouble` (`self.Boss Spawn Tile`))))
  (switch `/Game/Blueprints/Gamemodes/E_TutorialState` (`self.TutorialState`)
    (:`NewEnumerator0`
      (`self.Add Floor Tile` "NewEnumerator0" :!label _label))
    (:`NewEnumerator10`
      (goto _label))
    (:`NewEnumerator1`
      (goto _label))
    (:`NewEnumerator2`
      (if _returnvalue
        (`self.Add Floor Tile` "NewEnumerator1")
        (else
          (goto _label))))
    (:`NewEnumerator6`
      (if _returnvalue
        (`self.Add Floor Tile` "NewEnumerator2")
        (else
          (goto _label))))
    (:`NewEnumerator4`
      (if _returnvalue
        (`self.Add Floor Tile` "NewEnumerator4")
        (else
          (goto _label))))
    (:`NewEnumerator9`
      (goto _label))
    (:`NewEnumerator7`
      (goto _label))
    (:`NewEnumerator11`
      (goto _label))
    (:`NewEnumerator8`
      (if (not (`self.EndOfLevel`))
        (goto _label)))))

(fn `UserConstructionScript`
  (`parent.UserConstructionScript`))