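; Game mode for the bike demo level, which builds a procedural tile track leading to a boss fight.
; NextFloorTile randomizes bends and obstacles, weighting one obstacle type by player health, and leaves tiles plain at the start and around the boss.
; Tick flashes a warning before spawning the boss by tile count, adds a split tile once it is destroyed, tops up health at 1, and reloads on R.
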(event `self.ReceiveBeginPlay`
  (`parent.ReceiveBeginPlay`)
  (for _ (range 9)
    (`self.Next Floor Tile`))
  (bind _asbike_game_instance (cast `BikeGameInstance` (`GameplayStatics.GetGameInstance`)))
  (`BikeGameInstance.SetMobileState` _asbike_game_instance 2)
  (bind _returnvalue (`GameplayStatics.SpawnSound2D` "/Game/SoundFiles/SoundtracksWAV/MainLevel.MainLevel" 1.0 1.0 0.0 null false false))
  (bind _output_get (set `self.Level` _returnvalue))
  (`AudioComponent.FadeIn` _output_get 3.0 1.0 0.0 "Linear"))

(event `self.ReceiveTick`
  (params (DeltaSeconds :type "Float (single-precision)"))
  (bind _returnvalue (`GameplayStatics.GetPlayerController` 0))
  (bind _bossreference (`self.BossReference`))
  (`parent.ReceiveTick` DeltaSeconds)
  (if (`PlayerController.WasInputKeyJustPressed` _returnvalue "R")
    (`GameplayStatics.OpenLevelBySoftObjectPtr` "/Game/Maps/Level_Demo.Level_Demo")
    (else
      (bind _asbp_bike_player_controller (cast `/Game/Blueprints/Player/BP_BikePlayerController` _returnvalue))
      (bind _level_widget_reference (`/Game/Blueprints/Player/BP_BikePlayerController.Level Widget Reference` _asbp_bike_player_controller))
      (if (`/Game/UserInterface/HUD/HUDLevel.InResults` _level_widget_reference)
        _
        (elif (!= (`BikeProjectPlayerController.GetPlayerHealth` _asbp_bike_player_controller) 1)
          (if (== _bossreference null)
            (if (== (`self.Current Tile Count`) (- (`self.Boss Spawn Tile`) 10))
              (`/Game/UserInterface/HUD/HUDLevel.Set Text Flash` _level_widget_reference true)
              (elif (== (`self.Current Tile Count`) (`self.Boss Spawn Tile`))
                (`self.Spawn Boss` 1 20.0 0.4 DeltaSeconds)
                (`/Game/UserInterface/HUD/HUDLevel.Set Text Flash` _level_widget_reference false)))
            (else
              (switch `EBossState` (`BikeBoss.GetBossEnum` _bossreference)
                (:`BSE_Defeated`
                  (bind _boss_destroyed (`self.Destroy Boss` DeltaSeconds))
                  (if _boss_destroyed
                    (`self.Add Split Tile`))))))
          (else
            (`BikeProjectPlayerController.IncPlayerHealth` _asbp_bike_player_controller true)))))))

(fn `Next Floor Tile`
  (locals (Bending :type Boolean :default false))
  (bind _boss_spawn_tile (`self.Boss Spawn Tile`))
  (bind _current_tile_count (`self.Current Tile Count`))
  (if (not (`self.EndOfLevel`))
    (`parent.Next Floor Tile`)
    (set `self.Progressed` (/ (`KismetMathLibrary.Conv_IntToDouble` _current_tile_count) (`KismetMathLibrary.Conv_IntToDouble` _boss_spawn_tile)))
    (if (and (== (`self.BossReference`) null) (>= (- _boss_spawn_tile 11) _current_tile_count) (> _current_tile_count 5))
      (bind _output_get (set `local.Bending` (`KismetMathLibrary.RandomBool`)))
      (if (and (>= (`self.Tiles Since Last Bend`) 15) _output_get)
        (`self.Add Floor Tile` "NewEnumerator0" _output_get)
        (elif (== (mod _current_tile_count 5) 0)
          (if (!= (`KismetMathLibrary.RandomIntegerInRange` 0 3) 0)
            (`self.Add Floor Tile` "NewEnumerator1")
            (else
              (bind _asbp_bike_player_controller (cast `/Game/Blueprints/Player/BP_BikePlayerController` (`GameplayStatics.GetPlayerController` 0)))
              (if (>= (`KismetMathLibrary.RandomIntegerInRange` -5 8) (`BikeProjectPlayerController.GetPlayerHealth` _asbp_bike_player_controller))
                (`self.Add Floor Tile` "NewEnumerator4")
                (else
                  (`self.Add Floor Tile` "NewEnumerator2")))))
          (else
            (`self.Add Floor Tile` "NewEnumerator0" :!label _label))))
      (else
        (goto _label)))))

(fn `UserConstructionScript`
  (`parent.UserConstructionScript`))