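; BP_Lighting_Setup is an art-side lighting actor that exposes post-process look controls as Blueprint variables.
; Its construction script builds a post-process settings struct from those variables and assigns it to NewVar0, covering color temperature, global and shadow grading, ambient cubemap and ambient occlusion.
; Exposure brightness limits are pinned to equal values, fixing auto exposure.
; The event graph has no active logic.
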(fn `UserConstructionScript`
  (set `PostProcessVolume.Settings` (make `PostProcessSettings` :`WhiteTemp` (`self.ColourTemp`) :`ColorSaturation` (`self.Saturation`) :`ColorContrast` (`self.Contrast`) :`ColorGamma` (`self.Gamma`) :`ColorSaturationShadows` (`self.ShadowSat`) :`ColorContrastShadows` (`self.ShadowCon`) :`ColorGammaShadows` (`self.ShadowGam`) :`AmbientCubemapTint` (`self.AmbientCubemapTInt`) :`AmbientCubemapIntensity` (`self.AmbientCubemapIntensity`) :`AmbientCubemap` (`self.AmbientCubemapTexture`) :`AutoExposureMinBrightness` 1.0 :`AutoExposureMaxBrightness` 1.0 :`AmbientOcclusionIntensity` (`self.AOIntensity`) :`AmbientOcclusionRadius` (`self.AORadius`)) (`self.NewVar_0`)))