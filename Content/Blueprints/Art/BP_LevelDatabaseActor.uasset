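; Level database actor intended to build hierarchical instanced mesh components for modular building ground floors, floors and roofs.
; MakeBuildingArrayPerColour creates a component per mesh, with dynamic brick colour and front-material slot parameters, and adds it to an output array.
; The Construction Script's loops over building colours and indices are disconnected and marked as non-working WIP, so nothing currently runs.
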(fn `Make Building Array Per Colour`
  (params (`Input Array` :type "Array of StaticMesh Object Reference") (`Output Array` :type "Array of HierarchicalInstancedStaticMeshComponent Object Reference") (Color :type "Color Structure") (Index :type Integer))
  ;[0.02611 1 0.06393] SET Ground Floor Mesh Array
  (for _index (range (`KismetArrayLibrary.Array_Length` `Input Array`))
    (bind _returnvalue (`AddComponent|NODE_AddHierarchicalInstancedStaticMeshComponent-0` :`bManualAttachment` true :`RelativeTransform` (`KismetMathLibrary.MakeTransform` (0.0 0.0 0.0))))
    (`SceneComponent.K2_AttachToComponent` _returnvalue (`self.DefaultSceneRoot`) "None" "KeepRelative" "KeepRelative" "KeepRelative" true)
    (`StaticMeshComponent.SetStaticMesh` _returnvalue (`|GetArrayItem` `Input Array` _index))
    (bind _returnvalue_2 (`PrimitiveComponent.CreateDynamicMaterialInstance` _returnvalue (`MeshComponent.GetMaterialIndex` _returnvalue "Bricks") "/Game/Materials/Tileables/M_Building_Brick_01.M_Building_Brick_01" "None"))
    (`MaterialInstanceDynamic.SetVectorParameterValue` _returnvalue_2 "Colour1" (`KismetMathLibrary.Conv_ColorToLinearColor` Color))
    (bind _returnvalue_3 (`PrimitiveComponent.CreateDynamicMaterialInstance` _returnvalue (`MeshComponent.GetMaterialIndex` _returnvalue "Building_Front") "/Game/Materials/Atlases/M_Building_Front_Manual.M_Building_Front_Manual" "None"))
    (`MaterialInstanceDynamic.SetVectorParameterValue` _returnvalue_3 "SlotNumber" (make `LinearColor` (`KismetMathLibrary.Conv_IntToDouble` (mod Index 4)) (- (/ (`KismetMathLibrary.Conv_IntToDouble` Index) 4.0) 0.5)))
    (`KismetArrayLibrary.Array_Add` `Output Array` _returnvalue)))

(fn `UserConstructionScript`)