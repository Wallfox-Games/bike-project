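; BP_Spline_Cylinder is a construction-script art actor that builds a spline mesh shape, likely a cable or pipe, with clip meshes along it.
; Exposed locations and tangents shape the spline, which is split by Spacing into spline mesh segments with uniform Thickness and scaled tangents.
; Small selects between two clip static meshes, placed at constant-velocity intervals set by ClipPoints.
; The clip loop runs inside the segment loop, so clips repeat for every segment.
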(fn `UserConstructionScript`
  (bind _clip_points (`self.Clip Points`))
  (bind _spline (`self.Spline`))
  (bind _spline_2 (`self.Spline`))
  (bind _spacing (`self.Spacing`))
  (bind _tangentscale (`self.TangentScale`))
  (bind _spline_3 (`self.Spline`))
  (bind _thickness (`self.Thickness`))
  (`SplineComponent.AddSplinePoint` _spline_2 (`self.EndLocation`) "Local" true)
  (`SplineComponent.SetTangentAtSplinePoint` _spline_2 1 (`self.MiddleTangent`) "World" true)
  (`SplineComponent.SetTangentAtSplinePoint` _spline_2 2 (`self.EndTangent`) "World" true)
  (`SplineComponent.SetLocationAtSplinePoint` _spline_2 1 (`self.MiddleLocation`) "Local" true)
  (for _index (range (+ (`.ReturnValue` (`KismetMathLibrary.FMod` (`SplineComponent.GetSplineLength` _spline) _spacing)) 1))
    (bind _returnvalue (`AddComponent|NODE_AddSplineMeshComponent-1` :`bManualAttachment` true))
    (`SplineMeshComponent.SetStartScale` _returnvalue _thickness true)
    (`SplineMeshComponent.SetEndScale` _returnvalue _thickness true)
    (`PrimitiveComponent.SetMaterial` _returnvalue 0 "/Game/Materials/ColourMaterials/M_LUT_Colour_ALLVERT.M_LUT_Colour_ALLVERT")
    (bind _returnvalue_2 (* _index _spacing))
    (bind _returnvalue_3 (+ _returnvalue_2 _spacing))
    (`SplineMeshComponent.SetStartAndEnd` _returnvalue (`SplineComponent.GetLocationAtDistanceAlongSpline` _spline _returnvalue_2 "World") (* (`SplineComponent.GetDirectionAtDistanceAlongSpline` _spline _returnvalue_2 "World") _tangentscale) (`SplineComponent.GetLocationAtDistanceAlongSpline` _spline _returnvalue_3 "World") (* (`SplineComponent.GetDirectionAtDistanceAlongSpline` _spline _returnvalue_3 "World") _tangentscale) true)
    (for _index_2 (range (+ _clip_points 1))
      (if (`self.Small?`)
        (bind _returnvalue_4 (`AddComponent|NODE_AddStaticMeshComponent-1`))
        (else
          (bind _returnvalue_5 (`AddComponent|NODE_AddStaticMeshComponent-0`))))
      (bind _returnvalue_6 (* _index_2 (/ (`SplineComponent.Duration` _spline_3) (`KismetMathLibrary.Conv_IntToDouble` _clip_points))))
      (`SceneComponent.K2_SetWorldLocationAndRotation` _returnvalue_5 (`SplineComponent.GetLocationAtTime` _spline_3 _returnvalue_6 "World" true) (`SplineComponent.GetRotationAtTime` _spline_3 _returnvalue_6 "World" true) false false)
      (`SceneComponent.K2_SetWorldLocationAndRotation` _returnvalue_4 (`SplineComponent.GetLocationAtTime` _spline_3 _returnvalue_6 "World" true) (`SplineComponent.GetRotationAtTime` _spline_3 _returnvalue_6 "World" true) false false))))