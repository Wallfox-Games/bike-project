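; BP_Road procedurally builds a street tile in its construction script: road, pavements, lampposts, random benches and temporary hero buildings, mirrored across the road.
; Grid macros place mostly instanced meshes, with pavement dimensions from MakeBase positioning the props and buildings.
; An optional background preview stacks random-height buildings from ground, floor and roof meshes supplied by BP_LevelDatabaseActor.
; Seed is reset from the clock's milliseconds, so building variation changes on each reconstruction.
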(fn `Make Background Buildings`
  (params (`Center Location` :type "Vector Structure") (`Pavement Scale` :type "Float (double-precision)"))
  (bind _bottom_floor_mesh_inst (`self.Bottom Floor Mesh Inst`))
  (bind _building_amount__x_ (`self.Building Amount (x)`))
  (bind (_min _max) (`StaticMeshComponent.GetLocalBounds` (`self.RoadMeshInstanced`)))
  (bind _returnvalue (`KismetMathLibrary.RandomIntegerInRange` 0 (- (`KismetArrayLibrary.Array_Length` _bottom_floor_mesh_inst) 1)))
  (bind _output (`|GetArrayItem` (`self.Roof Mesh Inst`) _returnvalue))
  (bind _output_2 (`|GetArrayItem` _bottom_floor_mesh_inst _returnvalue))
  (bind _output_3 (`|GetArrayItem` (`self.Main Floor Mesh Inst`) _returnvalue))
  (bind (_current_point _total_points _0_1_phase _poly_center) (`/Engine/ArtTools/RenderToTexture/Macros/RenderToTextureMacros.2D Grid Execution Macro` (/ (* (`self.Tile Size`) 100.0) (`KismetMathLibrary.Conv_IntToDouble` _building_amount__x_)) (`KismetMathLibrary.MakeVector` (.x `Center Location`) (+ (+ (+ (.y `Center Location`) (`self.Lamppost Offset (Y)`)) (* (/ (`self.Tile Size`) (`KismetMathLibrary.Conv_IntToDouble` (`self.Pavement Sections`))) (* (`self.Pavement Y Sections`) 50.0))) (`KismetMathLibrary.Conv_IntToDouble` (* (`self.Building Offset`) 50))) (.z `Center Location`)) _building_amount__x_ (* (`self.Pavement Y Sections`) 4))
    (:`Per Poly Execution`
      (bind _x (.x _poly_center))
      (bind _y (.y _poly_center))
      (bind _returnvalue_2 (+ (.z _poly_center) (+ (* (/ (/ (`self.Tile Size`) (`KismetMathLibrary.Conv_IntToDouble` (`self.Pavement Sections`))) (* (.x (- _max _min)) 0.05)) 10.0) (`self.Pavement Z Offset`))))
      (`self.Place Buildings` _output_2 _output_3 _output (`KismetMathLibrary.MakeVector` _x _y _returnvalue_2) (struct :`Yaw` -90.0))
      (`self.Place Buildings` _output_2 _output_3 _output (`KismetMathLibrary.MakeVector` _x (* _y -1.0) _returnvalue_2) (struct :`Yaw` 90.0)))))

(fn `Make Base`
  (returns (`Pavement Location` :type "Vector Structure") (`Pavement Scale` :type "Float (double-precision)"))
  (bind _road_sections (`self.Road Sections`))
  (bind _returnvalue (/ (`self.Tile Size`) (`KismetMathLibrary.Conv_IntToDouble` _road_sections)))
  (bind _returnvalue_2 (* (`KismetMathLibrary.Conv_IntToDouble` (+ (`self.Pavement Y Sections`) 1)) _returnvalue))
  (bind _returnvalue_3 (* 50.0 (* _road_sections _returnvalue)))
  (`self.Make Pavement`)
  (bind (_current_point _total_points _0_1_phase _poly_center) (`/Engine/ArtTools/RenderToTexture/Macros/RenderToTextureMacros.2D Grid Execution Macro` (* _returnvalue 100.0) (`KismetMathLibrary.MakeVector` _returnvalue_3) _road_sections 1)
    (:`Per Poly Execution`
      (`InstancedStaticMeshComponent.AddInstance` (`self.RoadMeshInstanced`) (`KismetMathLibrary.MakeTransform` _poly_center (struct :`Yaw` 90.0) (`KismetMathLibrary.MakeVector` _returnvalue _returnvalue 1.0)))
      (switch `int` (- (`self.Road Sections`) _current_point)
        (:`1`
          (return (`KismetMathLibrary.MakeVector` _returnvalue_3 (* (- (+ _returnvalue _returnvalue_2) (`self.Pavement Bleed`)) 50.0)) _returnvalue_2))))))

(fn `Make Lampposts`
  (params (`Center Location` :type "Vector Structure") (`Pavement Scale` :type "Float (double-precision)"))
  (bind _lampost_amount (`self.Lampost Amount`))
  (bind _lamppostmeshinstanced (`self.LamppostMeshInstanced`))
  (bind _lamppost_scale (`self.Lamppost Scale`))
  (bind _returnvalue (`KismetMathLibrary.MakeVector` _lamppost_scale _lamppost_scale _lamppost_scale))
  (bind (_min _max) (`StaticMeshComponent.GetLocalBounds` (`self.RoadMeshInstanced`)))
  (bind (_current_point _total_points _0_1_phase _poly_center) (`/Engine/ArtTools/RenderToTexture/Macros/RenderToTextureMacros.2D Grid Execution Macro` (/ (* (`self.Tile Size`) 100.0) (`KismetMathLibrary.Conv_IntToDouble` _lampost_amount)) `Center Location` _lampost_amount 1)
    (:`Per Poly Execution`
      (bind _x (.x _poly_center))
      (bind _returnvalue_2 (+ (.y _poly_center) (+ (`self.Lamppost Offset (Y)`) (- 0.0 (* `Pavement Scale` 50.0)))))
      (bind _returnvalue_3 (+ (.z _poly_center) (+ (`self.Pavement Z Offset`) (* (/ (/ (`self.Tile Size`) (`KismetMathLibrary.Conv_IntToDouble` (`self.Pavement Sections`))) (* (.x (- _max _min)) 0.05)) 10.0))))
      (`InstancedStaticMeshComponent.AddInstance` _lamppostmeshinstanced (`KismetMathLibrary.MakeTransform` (`KismetMathLibrary.MakeVector` _x _returnvalue_2 _returnvalue_3) (struct) _returnvalue))
      (`InstancedStaticMeshComponent.AddInstance` _lamppostmeshinstanced (`KismetMathLibrary.MakeTransform` (`KismetMathLibrary.MakeVector` _x (* _returnvalue_2 -1.0) _returnvalue_3) (struct :`Yaw` -180.0) _returnvalue)))))

(fn `Make Pavement`
  (bind _pavement_sections (`self.Pavement Sections`))
  (bind _tile_size (`self.Tile Size`))
  (bind (_min _max) (`StaticMeshComponent.GetLocalBounds` (`self.RoadMeshInstanced`)))
  (bind _returnvalue (/ _tile_size (`KismetMathLibrary.Conv_IntToDouble` _pavement_sections)))
  (bind _returnvalue_2 (/ _returnvalue (* (.x (- _max _min)) 0.05)))
  (bind _returnvalue_3 (`KismetMathLibrary.MakeVector` _returnvalue_2 _returnvalue_2 _returnvalue_2))
  (bind (_current_point _total_points _0_1_phase _poly_center) (`/Engine/ArtTools/RenderToTexture/Macros/RenderToTextureMacros.2D Grid Execution Macro` (* _returnvalue 100.0) (`KismetMathLibrary.MakeVector` (* _tile_size 50.0)) _pavement_sections 1)
    (:`Per Poly Execution`
      (bind _returnvalue_4 (`KismetMathLibrary.MakeVector` (.x _poly_center) (+ (.y _poly_center) (* (- (+ _returnvalue (/ _tile_size (`KismetMathLibrary.Conv_IntToDouble` (`self.Road Sections`)))) (`self.Pavement Bleed`)) 50.0)) (+ (.z _poly_center) (`self.Pavement Z Offset`))))
      (`InstancedStaticMeshComponent.AddInstance` (`self.PavementInstancedStaticMesh`) (`KismetMathLibrary.MakeTransform` _returnvalue_4 (struct :`Yaw` -90.0) _returnvalue_3))
      (`self.Pavement Tiles` _returnvalue_4 1.0)
      (`InstancedStaticMeshComponent.AddInstance` (`self.PavementInstancedStaticMesh`) (`KismetMathLibrary.MakeTransform` (`KismetMathLibrary.MakeVector` (.x _returnvalue_4) (* (.y _returnvalue_4) -1.0) (.z _returnvalue_4)) (struct :`Yaw` 90.0) _returnvalue_3))
      (`self.Pavement Tiles` _returnvalue_4 -1.0))))

(fn `MakeBenches`
  (params (`Center Location` :type "Vector Structure") (`Pavement Scale` :type "Float (double-precision)"))
  (bind _bench_seed (`self.Bench Seed`))
  (bind _bench_density (`self.Bench Density`))
  (bind _bench_seed_2 (`self.Bench Seed`))
  (bind (_min _max) (`StaticMeshComponent.GetLocalBounds` (`self.RoadMeshInstanced`)))
  (bind _returnvalue (* (`self.Tile Size`) 100.0))
  (bind _returnvalue_2 (/ _returnvalue (* _bench_density 2.0)))
  (bind _returnvalue_3 (/ _returnvalue (* _bench_density 2.0)))
  (bind _returnvalue_4 (+ (* (/ (/ (`self.Tile Size`) (`KismetMathLibrary.Conv_IntToDouble` (`self.Pavement Sections`))) (* (.x (- _max _min)) 0.05)) 10.0) (`self.Pavement Z Offset`)))
  (bind (_current_point _total_points _0_1_phase _poly_center) (`/Engine/ArtTools/RenderToTexture/Macros/RenderToTextureMacros.2D Grid Execution Macro` (/ _returnvalue (`KismetMathLibrary.Conv_IntToDouble` _bench_density)) `Center Location` _bench_density 1)
    (:`Per Poly Execution`
      (if (`KismetMathLibrary.Conv_IntToBool` (`KismetMathLibrary.RandomIntegerInRangeFromStream` 0 1 _bench_seed_2))
        (`InstancedStaticMeshComponent.AddInstance` (`self.BenchMeshInstanced`) (`KismetMathLibrary.MakeTransform` (`KismetMathLibrary.MakeVector` (+ (.x _poly_center) (`KismetMathLibrary.RandomFloatInRangeFromStream` (* _returnvalue_3 -1.0) _returnvalue_3 _bench_seed_2)) (+ (.y _poly_center) (+ (`self.Bench Offset`) (- 0.0 (* `Pavement Scale` 50.0)))) (+ (+ (.z _poly_center) _returnvalue_4) (`self.Bench Vertical Offset`))) (struct :`Yaw` -90.0))))
      (if (`KismetMathLibrary.Conv_IntToBool` (`KismetMathLibrary.RandomIntegerInRangeFromStream` 0 1 _bench_seed))
        (`InstancedStaticMeshComponent.AddInstance` (`self.BenchMeshInstanced`) (`KismetMathLibrary.MakeTransform` (`KismetMathLibrary.MakeVector` (+ (.x _poly_center) (`KismetMathLibrary.RandomFloatInRangeFromStream` (* _returnvalue_2 -1.0) _returnvalue_2 _bench_seed)) (* (+ (.y _poly_center) (+ (`self.Bench Offset`) (- 0.0 (* `Pavement Scale` 50.0)))) -1.0) (+ (+ (.z _poly_center) _returnvalue_4) (`self.Bench Vertical Offset`))) (struct :`Yaw` 90.0)))))))

(fn `MakeBuildingArrayPerColour`
  (params (`Input Mesh Array` :type "Array of StaticMesh Object Reference") (`Output Mesh Array` :type "Array of HierarchicalInstancedStaticMeshComponent Object Reference") (`Building Colour` :type "LinearColor Structure") (Index :type Integer))
  ;[0.02611 1 0.06393] SET Ground Floor Mesh Array
  (for _index (range (`KismetArrayLibrary.Array_Length` `Input Mesh Array`))
    (bind _returnvalue (`AddComponent|NODE_AddHierarchicalInstancedStaticMeshComponent-2` :`bManualAttachment` true :`RelativeTransform` (`KismetMathLibrary.MakeTransform` (0.0 0.0 0.0))))
    (`SceneComponent.K2_AttachToComponent` _returnvalue (`self.DefaultSceneRoot`) "None" "KeepRelative" "KeepRelative" "KeepRelative" true)
    (`StaticMeshComponent.SetStaticMesh` _returnvalue (`|GetArrayItem` `Input Mesh Array` _index))
    (bind _returnvalue_2 (`PrimitiveComponent.CreateDynamicMaterialInstance` _returnvalue (`MeshComponent.GetMaterialIndex` _returnvalue "Bricks") "/Game/Materials/Tileables/M_BackgroundBuldingTemp.M_BackgroundBuldingTemp" "None"))
    (`MaterialInstanceDynamic.SetVectorParameterValue` _returnvalue_2 "Colour1" `Building Colour`)
    (bind _returnvalue_3 (`PrimitiveComponent.CreateDynamicMaterialInstance` _returnvalue (`MeshComponent.GetMaterialIndex` _returnvalue "Building_Front") "/Game/Materials/Atlases/M_Building_Front_Main.M_Building_Front_Main" "None"))
    (`MaterialInstanceDynamic.SetVectorParameterValue` _returnvalue_3 "SlotNumber" (make `LinearColor` (`KismetMathLibrary.Conv_IntToDouble` (mod Index 4)) (- (/ (`KismetMathLibrary.Conv_IntToDouble` Index) 4.0) 0.5)))
    (`KismetArrayLibrary.Array_Add` `Output Mesh Array` _returnvalue)))

(fn `MakeBuildingArrayPerColourMaterialSwitch`
  (params (`Input Array` :type "Array of StaticMesh Object Reference") (`Output Array` :type "Array of InstancedStaticMeshComponent Object Reference"))
  (for _array_element `Input Array`
    (bind _returnvalue (`AddComponent|NODE_AddInstancedStaticMeshComponent-1` :`bManualAttachment` true :`RelativeTransform` (`KismetMathLibrary.MakeTransform` (0.0 0.0 0.0))))
    (`SceneComponent.K2_AttachToComponent` _returnvalue (`self.DefaultSceneRoot`) "None" "KeepRelative" "KeepRelative" "KeepRelative" true)
    (`StaticMeshComponent.SetStaticMesh` _returnvalue _array_element)
    (`KismetArrayLibrary.Array_Add` `Output Array` _returnvalue)))

(fn `Pavement Tiles`
  (params (`Point Position` :type "Vector Structure") (direction :type "Float (double-precision)"))
  (bind _pavement_y_sections (`self.Pavement Y Sections`))
  (bind _returnvalue (/ (`self.Tile Size`) (`KismetMathLibrary.Conv_IntToDouble` (`self.Pavement Sections`))))
  (switch `int` _pavement_y_sections
    (:`Default`
      (for _index (range _pavement_y_sections)
        (bind _returnvalue_2 (`AddComponent|NODE_AddStaticMeshComponent-7` :`RelativeTransform` (`KismetMathLibrary.MakeTransform` (`KismetMathLibrary.MakeVector` (.x `Point Position`) (* (+ (* (* (+ _index 1) _returnvalue) 100.0) (.y `Point Position`)) direction) (- (`self.Pavement Z Offset`) 8.0)) (struct) (`KismetMathLibrary.MakeVector` _returnvalue _returnvalue 0.2))))
        (`StaticMeshComponent.SetStaticMesh` _returnvalue_2 "/Game/Meshes/Shapes/Shape_Cube.Shape_Cube")
        (`PrimitiveComponent.SetMaterial` _returnvalue_2 0 (`self.Pavement Tile Material`))))
    (:`0`
      _))
  (return))

(fn `Pick Buildings`
  (params (`Ground Floor` :type "StaticMesh Object Reference") (Floor :type "StaticMesh Object Reference") (Roof :type "StaticMesh Object Reference") (`Ground Window Material` :type "MaterialInstance Object Reference") (`Floor Window Material` :type "MaterialInstance Object Reference") (`Brick Material` :type "MaterialInstance Object Reference"))
  (returns (`Ground Floor inst` :type "HierarchicalInstancedStaticMeshComponent Object Reference") (`Floor Inst` :type "HierarchicalInstancedStaticMeshComponent Object Reference") (`Roof Inst` :type "HierarchicalInstancedStaticMeshComponent Object Reference"))
  (bind _returnvalue (`AddComponent|NODE_AddHierarchicalInstancedStaticMeshComponent-3` :`bManualAttachment` true :`RelativeTransform` (`KismetMathLibrary.MakeTransform` (0.0 0.0 0.0))))
  (`SceneComponent.K2_AttachToComponent` _returnvalue (`self.DefaultSceneRoot`) "None" "KeepRelative" "KeepRelative" "KeepRelative" true)
  (`StaticMeshComponent.SetStaticMesh` _returnvalue `Ground Floor`)
  (`PrimitiveComponent.SetMaterial` _returnvalue (`MeshComponent.GetMaterialIndex` _returnvalue "Bricks") `Brick Material`)
  (`PrimitiveComponent.SetMaterial` _returnvalue (`MeshComponent.GetMaterialIndex` _returnvalue "Building_Front") `Ground Window Material`)
  (bind _returnvalue_2 (`AddComponent|NODE_AddHierarchicalInstancedStaticMeshComponent-4` :`bManualAttachment` true :`RelativeTransform` (`KismetMathLibrary.MakeTransform` (0.0 0.0 0.0))))
  (`SceneComponent.K2_AttachToComponent` _returnvalue_2 (`self.DefaultSceneRoot`) "None" "KeepRelative" "KeepRelative" "KeepRelative" true)
  (`StaticMeshComponent.SetStaticMesh` _returnvalue_2 Floor)
  (`PrimitiveComponent.SetMaterial` _returnvalue_2 (`MeshComponent.GetMaterialIndex` _returnvalue_2 "Bricks") `Brick Material`)
  (`PrimitiveComponent.SetMaterial` _returnvalue_2 (`MeshComponent.GetMaterialIndex` _returnvalue_2 "Building_Front") `Floor Window Material`)
  (bind _returnvalue_3 (`AddComponent|NODE_AddHierarchicalInstancedStaticMeshComponent-5` :`bManualAttachment` true :`RelativeTransform` (`KismetMathLibrary.MakeTransform` (0.0 0.0 0.0))))
  (`SceneComponent.K2_AttachToComponent` _returnvalue_3 (`self.DefaultSceneRoot`) "None" "KeepRelative" "KeepRelative" "KeepRelative" true)
  (`StaticMeshComponent.SetStaticMesh` _returnvalue_3 Roof)
  (`PrimitiveComponent.SetMaterial` _returnvalue_3 (`MeshComponent.GetMaterialIndex` _returnvalue_3 "Bricks") `Brick Material`)
  (`PrimitiveComponent.SetMaterial` _returnvalue_3 (`MeshComponent.GetMaterialIndex` _returnvalue_3 "Building_Front") `Floor Window Material`)
  (return _returnvalue _returnvalue_2 _returnvalue_3))

(fn `Place Buildings`
  (params (`Ground Floor Mesh` :type "InstancedStaticMeshComponent Object Reference") (`Floor Mesh` :type "InstancedStaticMeshComponent Object Reference") (`Roof Mesh` :type "InstancedStaticMeshComponent Object Reference") (`Point Location` :type "Vector Structure") (Rotation :type "Rotator Structure"))
  (bind (_min _max) (`StaticMeshComponent.GetLocalBounds` `Ground Floor Mesh`))
  (bind _building_scale (`self.Building Scale`))
  (bind _max_floors (`self.Max Floors`))
  (bind _building_scale_2 (`self.Building Scale`))
  (bind _returnvalue (`KismetMathLibrary.MakeVector` _building_scale _building_scale _building_scale))
  (bind _returnvalue_2 (`KismetMathLibrary.RandomIntegerInRangeFromStream` (`self.Min Floors`) _max_floors (`self.Seed`)))
  (bind _z (.z (* _max _building_scale_2)))
  (bind _returnvalue_3 (`KismetMathLibrary.MakeVector` (.x `Point Location`) (.y `Point Location`) (+ (.z `Point Location`) _z)))
  (`InstancedStaticMeshComponent.AddInstance` `Ground Floor Mesh` (`KismetMathLibrary.MakeTransform` _returnvalue_3 Rotation _returnvalue))
  (switch `int` _max_floors
    (:`Default`
      (for _index (range _returnvalue_2)
        (switch `int` _returnvalue_2
          (:`Default`
            (bind _returnvalue_4 (`KismetMathLibrary.MakeVector` (.x _returnvalue_3) (.y _returnvalue_3) (+ (.z _returnvalue_3) (* (+ _index 1) (- _z (.z (* _min _building_scale_2)))))))
            (`InstancedStaticMeshComponent.AddInstance` `Floor Mesh` (`KismetMathLibrary.MakeTransform` _returnvalue_4 Rotation _returnvalue)))
          (:`0`
            (`InstancedStaticMeshComponent.AddInstance` `Roof Mesh` (`KismetMathLibrary.MakeTransform` (`KismetMathLibrary.MakeVector` (.x _returnvalue_4) (.y _returnvalue_4) (.z _returnvalue_4)) Rotation _returnvalue) :!label _label)
            (return)))))
    (:`0`
      _))
  (goto _label))

(fn `TEMP_Herobuildings`
  (params (`Center Position` :type "Vector Structure"))
  (bind _hero_building_amount__temp_ (`self.Hero Building Amount [TEMP]`))
  (bind _returnvalue (`KismetMathLibrary.RandomFloatInRangeFromStream` 0.9 1.1 (`self.Seed`)))
  (bind (_min _max) (`StaticMeshComponent.GetLocalBounds` (`self.RoadMeshInstanced`)))
  (bind _returnvalue_2 (`KismetMathLibrary.MakeVector` _returnvalue _returnvalue _returnvalue))
  (bind (_current_point _total_points _0_1_phase _poly_center) (`/Engine/ArtTools/RenderToTexture/Macros/RenderToTextureMacros.2D Grid Execution Macro` (/ (* (`self.Tile Size`) 100.0) (`KismetMathLibrary.Conv_IntToDouble` _hero_building_amount__temp_)) `Center Position` _hero_building_amount__temp_ 1)
    (:`Per Poly Execution`
      (bind _x (.x _poly_center))
      (bind _returnvalue_3 (+ (.y _poly_center) (* (`self.Hero Building Offset [TEMP]`) 10.0)))
      (bind _returnvalue_4 (+ 8.0 (+ (.z _poly_center) (* (/ (/ (`self.Tile Size`) (`KismetMathLibrary.Conv_IntToDouble` (`self.Pavement Sections`))) (* (.x (- _max _min)) 0.05)) 10.0))))
      (bind _returnvalue_5 (`AddComponent|NODE_AddStaticMeshComponent-8` :`RelativeTransform` (`KismetMathLibrary.MakeTransform` (`KismetMathLibrary.MakeVector` _x _returnvalue_3 _returnvalue_4) (struct) _returnvalue_2)))
      (`StaticMeshComponent.SetStaticMesh` _returnvalue_5 "/Game/Meshes/Hero_Buildings/SM_Hero_Building_01_-_Copy.SM_Hero_Building_01_-_Copy")
      (bind _returnvalue_6 (`AddComponent|NODE_AddStaticMeshComponent-9` :`RelativeTransform` (`KismetMathLibrary.MakeTransform` (`KismetMathLibrary.MakeVector` _x (* _returnvalue_3 -1.0) _returnvalue_4) (struct :`Yaw` 180.0) _returnvalue_2)))
      (`StaticMeshComponent.SetStaticMesh` _returnvalue_6 "/Game/Meshes/Hero_Buildings/SM_Hero_Building_01_-_Copy.SM_Hero_Building_01_-_Copy"))))

(fn `UserConstructionScript`
  (bind _pavementinstancedstaticmesh (`self.PavementInstancedStaticMesh`))
  (`KismetMathLibrary.SetRandomStreamSeed` (`self.Seed`) (`KismetMathLibrary.GetMillisecond` (`KismetMathLibrary.Now`)))
  (bind _returnvalue (`GameplayStatics.GetActorOfClass` "/Game/Blueprints/Art/BP_LevelDatabaseActor.BP_LevelDatabaseActor_C"))
  (set `self.Bottom Floor Mesh` (`/Game/Blueprints/Art/BP_LevelDatabaseActor.Ground Floor Mesh` _returnvalue))
  (set `self.Main Floor Mesh` (`/Game/Blueprints/Art/BP_LevelDatabaseActor.Floor Mesh` _returnvalue))
  (set `self.Roof Mesh` (`/Game/Blueprints/Art/BP_LevelDatabaseActor.Roof Mesh` _returnvalue))
  (`self.MakeBuildingArrayPerColourMaterialSwitch` (`self.Bottom Floor Mesh`) (`self.Bottom Floor Mesh Inst`))
  (`self.MakeBuildingArrayPerColourMaterialSwitch` (`self.Main Floor Mesh`) (`self.Main Floor Mesh Inst`))
  (`self.MakeBuildingArrayPerColourMaterialSwitch` (`self.Roof Mesh`) (`self.Roof Mesh Inst`))
  (`StaticMeshComponent.SetStaticMesh` (`self.RoadMeshInstanced`) "/Game/Meshes/Shapes/Shape_Plane.Shape_Plane")
  (`PrimitiveComponent.SetMaterial` (`self.RoadMeshInstanced`) 0 (`self.Road Material`))
  (`StaticMeshComponent.SetStaticMesh` (`self.BenchMeshInstanced`) (`self.Bench Mesh`))
  (`StaticMeshComponent.SetStaticMesh` (`self.LamppostMeshInstanced`) (`self.Lamppost Mesh`))
  (`PrimitiveComponent.SetMaterial` (`self.LamppostMeshInstanced`) 0 (`self.Lamppost Material`))
  (`StaticMeshComponent.SetStaticMesh` (`self.PavementInstancedStaticMesh`) (`self.Pavement Mesh`))
  (`PrimitiveComponent.SetMaterial` _pavementinstancedstaticmesh 0 (`self.Pavement Trim Material`))
  (`PrimitiveComponent.SetMaterial` _pavementinstancedstaticmesh 1 (`self.Pavement Tile Material`))
  (bind (_pavement_location _pavement_scale) (`self.Make Base`))
  (`self.Make Lampposts` _pavement_location _pavement_scale)
  (`self.MakeBenches` _pavement_location _pavement_scale)
  (if (`self.Enable Background Buildings (Preview)`)
    (`self.Make Background Buildings` _pavement_location _pavement_scale))
  (`self.TEMP_Herobuildings` _pavement_location))