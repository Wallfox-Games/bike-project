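; Destructible obstacle that shatters when the player character hits it.
; Hit applies radius damage at the impact point, with impulse scaled by the player's power percent, plus optional explosion particles and sound.
; It then calls OnHit on the BP_ObstacleChecker it is attached to and switches the destructible to physics-only collision; without that parent, collision stays unchanged.
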(event `self.ReceiveHit`
  (params (MyComp :type "PrimitiveComponent Object Reference") (Other :type "Actor Object Reference") (OtherComp :type "PrimitiveComponent Object Reference") (bSelfMoved :type Boolean) (HitLocation :type "Vector Structure") (HitNormal :type "Vector Structure") (NormalImpulse :type "Vector Structure") (Hit :type "HitResult Structure (by ref)"))
  (bind _destructible (`self.Destructible`))
  (bind _returnvalue (`SceneComponent.K2_GetComponentLocation` _destructible))
  (bind _asbp_player_character (cast `/Game/Blueprints/Player/BP_PlayerCharacter` Other))
  (`DestructibleComponent.ApplyRadiusDamage` _destructible 500.0 HitLocation 500.0 (+ (`self.PowerAddition`) (* (`BikeCharacter.GetPowerPercent` _asbp_player_character) (`self.PowerScaling`))) true)
  (if (`self.UseParticles?`)
    (`GameplayStatics.SpawnEmitterAtLocation` "/Game/ParticleSystems/P_Explosion_01.P_Explosion_01" (+ _returnvalue (200.0 0.0 0.0))))
  (if (`self.PlaySound?`)
    (`GameplayStatics.PlaySoundAtLocation` (`self.Sound`) _returnvalue (struct) (`self.VolumeMultiplier`) (`self.PitchMultiplier`) 0.0 null null null))
  (bind _asbp_obstacle_checker (cast `/Game/Blueprints/Tiles/BP_ObstacleChecker` (`ActorComponent.GetOwner` (`SceneComponent.GetAttachParent` (`self.DefaultSceneRoot`)))))
  (`/Game/Blueprints/Tiles/BP_ObstacleChecker.OnHit` _asbp_obstacle_checker)
  (`PrimitiveComponent.SetCollisionEnabled` (`self.Destructible`) "PhysicsOnly"))

(fn `UserConstructionScript`)