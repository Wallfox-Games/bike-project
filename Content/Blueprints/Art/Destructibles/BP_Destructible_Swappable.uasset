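; BP_Destructible_Swappable is a destructible prop that swaps its static mesh for a hidden Destructible component when hit.
; For player character hits, it applies radius damage at the hit point, with impulse scaled by the player's power percent.
; It optionally spawns an explosion particle, then notifies the owning BP_ObstacleBase through its attachment parent chain.
; Once that obstacle is notified, the destructible's collision becomes physics-only.
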(event `self.ReceiveHit`
  (params (MyComp :type "PrimitiveComponent Object Reference") (Other :type "Actor Object Reference") (OtherComp :type "PrimitiveComponent Object Reference") (bSelfMoved :type Boolean) (HitLocation :type "Vector Structure") (HitNormal :type "Vector Structure") (NormalImpulse :type "Vector Structure") (Hit :type "HitResult Structure (by ref)"))
  (bind _destructible (`self.Destructible`))
  (`SceneComponent.SetVisibility` (`self.StaticMesh`) false false)
  (`SceneComponent.SetVisibility` (`self.Destructible`) true false)
  (bind _asbp_player_character (cast `/Game/Blueprints/Player/BP_PlayerCharacter` Other))
  (`DestructibleComponent.ApplyRadiusDamage` _destructible 500.0 HitLocation 500.0 (+ (* (`BikeCharacter.GetPowerPercent` _asbp_player_character) (`self.PowerScaling`)) (`self.PowerAddition`)) true)
  (if (`self.UseParticles?`)
    (`GameplayStatics.SpawnEmitterAtLocation` "/Game/ParticleSystems/P_Explosion_01.P_Explosion_01" (+ (`SceneComponent.K2_GetComponentLocation` _destructible) (200.0 0.0 0.0))))
  (bind _asbp_obstacle_base (cast `/Game/Blueprints/Tiles/Add-ons/BP_ObstacleBase` (`self.GetParentActor` (`ActorComponent.GetOwner` (`SceneComponent.GetAttachParent` (`self.DefaultSceneRoot`))))))
  (`/Game/Blueprints/Tiles/Add-ons/BP_ObstacleBase.On Hit` _asbp_obstacle_base)
  (`PrimitiveComponent.SetCollisionEnabled` (`self.Destructible`) "PhysicsOnly"))

(fn `UserConstructionScript`)