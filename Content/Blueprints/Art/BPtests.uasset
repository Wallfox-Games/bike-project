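; BPtests is a test Blueprint that shows one of two cube positions based on the LRToggle flag.
; Its construction script creates a hierarchical instanced static mesh component with the cube mesh and adds two instances, one at the origin and one offset along Y.
; It then removes one by its returned index: the origin instance when LRToggle is true, otherwise the offset one.
; The event graph is empty.
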(fn `UserConstructionScript`
  (bind _returnvalue (`AddComponent|NODE_AddHierarchicalInstancedStaticMeshComponent-0` :`RelativeTransform` (`KismetMathLibrary.MakeTransform` (0.0 0.0 0.0))))
  (`StaticMeshComponent.SetStaticMesh` _returnvalue "/Game/Meshes/Shapes/Shape_Cube.Shape_Cube")
  (bind _returnvalue_2 (`InstancedStaticMeshComponent.AddInstance` _returnvalue (`KismetMathLibrary.MakeTransform` (0.0 0.0 0.0))))
  (bind _returnvalue_3 (`InstancedStaticMeshComponent.AddInstance` _returnvalue (`KismetMathLibrary.MakeTransform` (0.0 60.0 0.0))))
  (if (`self.LR Toggle`)
    (`InstancedStaticMeshComponent.RemoveInstance` _returnvalue _returnvalue_2)
    (else
      (`InstancedStaticMeshComponent.RemoveInstance` _returnvalue _returnvalue_3))))