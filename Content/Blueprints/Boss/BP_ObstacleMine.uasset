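; Mine obstacle Blueprint, filed under Boss, that penalizes the bike player when hit.
; Its On Hit override, skipped if ActivatedOnHit is set, calls ChangeComboMeter and PlayerHit with false on the first player's BP_BikePlayerController, then runs the parent's hit logic.
; Despawn simply destroys the actor, and the event graph holds only disabled default events.
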(fn `Despawn`
  (`self.K2_DestroyActor`))

(fn `On Hit`
  (if (not (`self.ActivatedOnHit`))
    (bind _asbp_bike_player_controller (cast `/Game/Blueprints/Player/BP_BikePlayerController` (`GameplayStatics.GetPlayerController` 0)))
    (`BikeProjectPlayerController.ChangeComboMeter` _asbp_bike_player_controller false)
    (`BikeProjectPlayerController.PlayerHit` _asbp_bike_player_controller false)
    (`parent.On Hit`)))

(fn `UserConstructionScript`
  (`parent.UserConstructionScript`))