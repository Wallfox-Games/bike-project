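; Boss actor for a bike game that loses health whenever the player character overlaps its box.
; Tick feeds two of the player's raw power readings into Movement as the player's level and max.
; Each overlap decrements boss health stored in BikeGameInstance and clears the player's attacking state while health remains.
; At zero it flags the boss defeated, swaps its visible component for a child actor, then destroys itself after a short delay.
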(event `self.ReceiveTick`
  (params (DeltaSeconds :type "Float (single-precision)"))
  (bind _asbp_player_character (cast `/Game/Blueprints/Player/BP_PlayerCharacter` (`GameplayStatics.GetPlayerPawn` 0)))
  (`self.Movement` (`BikeCharacter.GetRawPower` _asbp_player_character 4) (`BikeCharacter.GetRawPower` _asbp_player_character 3)))

(event `self.Box.OnComponentBeginOverlap`
  (params (OverlappedComponent :type "PrimitiveComponent Object Reference") (OtherActor :type "Actor Object Reference") (OtherComp :type "PrimitiveComponent Object Reference") (OtherBodyIndex :type Integer) (bFromSweep :type Boolean) (SweepResult :type "HitResult Structure (by ref)"))
  (bind _returnvalue (`GameplayStatics.GetGameInstance`))
  (cast `/Game/Blueprints/Player/BP_PlayerCharacter` OtherActor)
  (bind _asbike_game_instance (cast `BikeGameInstance` _returnvalue))
  (bind _result (`/Engine/EditorBlueprintResources/StandardMacros.DecrementInt` (`BikeGameInstance.GetBossHealth` _asbike_game_instance))
    (:`  `
      (`BikeGameInstance.SetBossHealth` _asbike_game_instance _result)
      (if (== (`BikeGameInstance.GetBossHealth` _asbike_game_instance) 0)
        (bind _asbike_game_instance_2 (cast `BikeGameInstance` _returnvalue))
        (`BikeGameInstance.SetBossDefeated` _asbike_game_instance_2 true)
        (`SceneComponent.SetVisibility` (`self.BossVisibleComponent`) false false)
        (`SceneComponent.SetVisibility` (`self.ChildActor`) true false)
        (`KismetSystemLibrary.Delay` 3.0)
        (`self.K2_DestroyActor`)
        (else
          (bind _asbp_player_character (cast `/Game/Blueprints/Player/BP_PlayerCharacter` (`GameplayStatics.GetPlayerPawn` 0)))
          (`BikeCharacter.SetAttacking` _asbp_player_character false))))))

(fn `UserConstructionScript`)