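; BP_BikeBoss is a bike-game boss that drops mines behind itself and breaks apart when the player lands the finishing hit.
; Parent-class state changes despawn mines and play or reverse a camera timeline around the vulnerable phase.
; Tick scales the player and a DinosaurGrowth material parameter with attack power while mines reload, shrinking the player during cooldown or defeat.
; Hits update the controller's boss reference and chunk count, swapping in a destructible mesh on success.
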(event `self.ReceiveBeginPlay`
  (`parent.ReceiveBeginPlay`))

(event `self.DestroySelf`
  (`parent.DestroySelf`)
  (`self.K2_DestroyActor`))

(event `self.ReceiveTick`
  (params (DeltaSeconds :type "Float (single-precision)"))
  (bind _returnvalue (`self.GetPercentageAttackPower`))
  (`parent.ReceiveTick` DeltaSeconds)
  (bind _asbp_player_character (cast `/Game/Blueprints/Player/BP_PlayerCharacter` (`GameplayStatics.GetPlayerPawn` 0)))
  (switch `EBossState` (`self.GetBossEnum`)
    (:`BSE_Cooldown`
      (bind _scale (`/Game/Blueprints/Player/BP_PlayerCharacter.Get Scale` _asbp_player_character :!label _label))
      (`/Game/Blueprints/Player/BP_PlayerCharacter.Set Scale` _asbp_player_character (`KismetMathLibrary.Conv_DoubleToVector` (`KismetMathLibrary.FClamp` (- _scale (* DeltaSeconds 2.0)) 0.8 2.5)))
      (`KismetMaterialLibrary.SetScalarParameterValue` "/Game/Materials/Material_Functions/MainParameterCollection.MainParameterCollection" "DinosaurGrowth"))
    (:`BSE_Reloading`
      (`/Game/Blueprints/Player/BP_PlayerCharacter.Set Scale` _asbp_player_character (`KismetMathLibrary.Conv_DoubleToVector` (+ (* _returnvalue 1.7) 0.8)))
      (`KismetMaterialLibrary.SetScalarParameterValue` "/Game/Materials/Material_Functions/MainParameterCollection.MainParameterCollection" "DinosaurGrowth" _returnvalue))
    (:`BSE_Defeated`
      (goto _label))))

(event `self.InitValues`
  (params (NewPtr :type "BikeCharacter Object Reference") (NewHealth :type Integer) (NewSeconds :type "Float (single-precision)") (NewMultiplier :type "Float (single-precision)") (DeltaTime :type "Float (single-precision)"))
  (`parent.InitValues` NewPtr NewHealth NewSeconds NewMultiplier DeltaTime)
  (bind _asbp_bike_player_controller (cast `/Game/Blueprints/Player/BP_BikePlayerController` (`GameplayStatics.GetPlayerController` 0)))
  (`/Game/UserInterface/HUD/HUDBoss.Init Values` (`/Game/Blueprints/Player/BP_BikePlayerController.Boss Reference` _asbp_bike_player_controller) self))

(event `self.ReceiveHit`
  (params (MyComp :type "PrimitiveComponent Object Reference") (Other :type "Actor Object Reference") (OtherComp :type "PrimitiveComponent Object Reference") (bSelfMoved :type Boolean) (HitLocation :type "Vector Structure") (HitNormal :type "Vector Structure") (NormalImpulse :type "Vector Structure") (Hit :type "HitResult Structure (by ref)"))
  (bind _bossdestructiblecomponent (`self.BossDestructibleComponent`))
  (cast `/Game/Blueprints/Player/BP_PlayerCharacter` Other)
  (bind _returnvalue (`self.OnHit`))
  (if _returnvalue
    (`GameplayStatics.PlaySoundAtLocation` "/Game/SoundFiles/SoundFilesWAV/DestructionImpactBossHit.DestructionImpactBossHit" HitLocation (struct) 1.0 1.0 0.0 null null null)
    (`SceneComponent.SetVisibility` (`self.BossVisibleComponent`) false false)
    (`SceneComponent.SetVisibility` _bossdestructiblecomponent true false)
    (`DestructibleComponent.ApplyRadiusDamage` _bossdestructiblecomponent 500.0 HitLocation 500.0 800.0 true)
    (`self.SetActorEnableCollision` false)
    (else
      (`GameplayStatics.PlaySoundAtLocation` "/Game/SoundFiles/SoundFilesWAV/DestructionImpactBossHit.DestructionImpactBossHit" HitLocation (struct) 1.0 1.0 0.0 null null null))))

(event `self.SpawnMine`
  (bind _rootcomponent (`self.RootComponent`))
  (`parent.SpawnMine`)
  (bind _returnvalue (`|SpawnActorFromClass` "/Game/Blueprints/Boss/BP_ObstacleMine.BP_ObstacleMine_C" (`KismetMathLibrary.MakeTransform` (+ (* (`SceneComponent.GetForwardVector` _rootcomponent) -150.0) (.location (`SceneComponent.K2_GetComponentToWorld` _rootcomponent)) (0.0 0.0 0.0)) (`KismetMathLibrary.ComposeRotators` (.rotation (`SceneComponent.K2_GetComponentToWorld` _rootcomponent)) (`KismetMathLibrary.RotatorFromAxisAndAngle` (0.0 0.0 1.0) 90.0)) (* (.scale (`SceneComponent.K2_GetComponentToWorld` _rootcomponent)) 3.0)) "AlwaysSpawn" "OverrideRootScale" null null))
  (`KismetArrayLibrary.Array_Insert` (`self.MinesArray`) _returnvalue))

(event `self.ChangeState`
  (params (NewState :type "EBossState Enum" :default "BSE_Moving"))
  (bind _bosscameraspringarm (`self.BossCameraSpringArm`))
  (`parent.ChangeState` NewState)
  (switch `EBossState` NewState
    (:`BSE_Cooldown`
      (bind (_direction _spring_arm_location _spring_arm_rotation _target_arm_length _fov _bossxoffset) (`Timeline|Camera Timeline` :!via `ReverseFromEnd` :!label _label_2)
        (:`Update`
          (set `SpringArmComponent.TargetArmLength` _target_arm_length _bosscameraspringarm)
          (`SceneComponent.K2_SetRelativeLocationAndRotation` _bosscameraspringarm _spring_arm_location (`KismetMathLibrary.MakeRotator` (.x _spring_arm_rotation) (.y _spring_arm_rotation) (.z _spring_arm_rotation)) false false)
          (`CameraComponent.SetFieldOfView` (`self.BossCamera`) _fov))))
    (:`BSE_Despawning`
      (for _array_element (`self.MinesArray`)
        (`/Game/Blueprints/Boss/BP_ObstacleMine.Despawn` _array_element))
      (set `self.ObstaclesDestroyed` true))
    (:`BSE_Vulnerable`
      (goto _label_2 :!via `PlayFromStart`))
    (:`BSE_Defeated`
      (goto _label_2 :!via `ReverseFromEnd`))))

(fn `OnHit`
  (returns (ReturnValue :type Boolean))
  (bind _returnvalue (`parent.OnHit`))
  (bind _asbp_bike_player_controller (cast `/Game/Blueprints/Player/BP_BikePlayerController` (`GameplayStatics.GetPlayerController` 0)))
  (`/Game/UserInterface/HUD/HUDBoss.Set Health` (`/Game/Blueprints/Player/BP_BikePlayerController.Boss Reference` _asbp_bike_player_controller))
  (bind _asbike_game_instance (cast `BikeGameInstance` (`GameplayStatics.GetGameInstance`)))
  (`BikeGameInstance.IncBossChunks` _asbike_game_instance)
  (return _returnvalue))

(fn `UserConstructionScript`)