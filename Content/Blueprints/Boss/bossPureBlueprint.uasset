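; Boss actor Blueprint that restarts play at Level_Main when it hits the player character.
; Tick sets Speed from a clamped power ratio using BikeGameInstance's max power, but the numerator is a literal zero, so it stays at the base value.
; A collision hit pauses the game, then calls a Delay before opening the level.
; No movement logic here consumes Speed.
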(event `self.ReceiveTick`
  (params (DeltaSeconds :type "Float (single-precision)"))
  (bind _asbike_game_instance (cast `BikeGameInstance` (`GameplayStatics.GetGameInstance`)))
  (cast `/Game/Blueprints/Player/BP_PlayerCharacter` (`GameplayStatics.GetPlayerPawn` 0))
  (set `self.Speed` (+ (* (`KismetMathLibrary.FClamp` (/ 0.0 (`BikeGameInstance.GetMaxPower` _asbike_game_instance))) 300.0) 200.0)))

(event `self.collision.OnComponentHit`
  (params (HitComponent :type "PrimitiveComponent Object Reference") (OtherActor :type "Actor Object Reference") (OtherComp :type "PrimitiveComponent Object Reference") (NormalImpulse :type "Vector Structure") (Hit :type "HitResult Structure (by ref)"))
  (cast `/Game/Blueprints/Player/BP_PlayerCharacter` OtherActor)
  (`GameplayStatics.SetGamePaused` true)
  (`KismetSystemLibrary.Delay` 2.0)
  (`GameplayStatics.OpenLevel` "Level_Main"))

(fn `UserConstructionScript`)