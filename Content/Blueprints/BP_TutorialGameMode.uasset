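; Tutorial game mode that builds a floor-tile track, shows four timed pop-ups, then loads Level_Main.
; A Delay on Tick drives a roughly once-per-second counter that triggers each pausing pop-up and the final level change.
; NextFloorTile, pre-run ten times at start, switches every third tile to another type after the second pop-up.
; Disconnected nodes hold unused player max-power calibration and debug prints.
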(event `self.ReceiveBeginPlay`
  (`parent.ReceiveBeginPlay`)
  (set `self.Current Power` 0.0)
  (set `self.Passed PopUp2` false)
  (set `self.Current Tile Count` 0)
  (for _ (range 10)
    (`self.Next Floor Tile`)))

(event `self.ReceiveTick`
  (params (DeltaSeconds :type "Float (single-precision)"))
  (`KismetSystemLibrary.Delay` 1.0)
  (if (== (`self.Seconds`) 45)
    (bind _returnvalue (`|CreateWidget` "/Game/UserInterface/PopUp1.PopUp1_C"))
    (bind _output_get (set `self.Pop Up 1 Ref` _returnvalue))
    (`UserWidget.AddToViewport` _output_get 0)
    (`GameplayStatics.SetGamePaused` true)
    (elif (== (`self.Seconds`) 90)
      (bind _returnvalue_2 (`|CreateWidget` "/Game/UserInterface/PopUp2.PopUp2_C"))
      (bind _output_get_2 (set `self.Pop Up 2 Ref` _returnvalue_2))
      (`UserWidget.AddToViewport` _output_get_2 0)
      (set `self.Passed PopUp2` true)
      (`GameplayStatics.SetGamePaused` true)
      (elif (== (`self.Seconds`) 135)
        (bind _returnvalue_3 (`|CreateWidget` "/Game/UserInterface/PopUp3.PopUp3_C"))
        (bind _output_get_3 (set `self.Pop Up 3 Ref` _returnvalue_3))
        (`UserWidget.AddToViewport` _output_get_3 0)
        (`GameplayStatics.SetGamePaused` true)
        (elif (== (`self.Seconds`) 180)
          (bind _returnvalue_4 (`|CreateWidget` "/Game/UserInterface/PopUp4.PopUp4_C"))
          (bind _output_get_4 (set `self.Pop Up 4 Ref` _returnvalue_4))
          (`UserWidget.AddToViewport` _output_get_4 0)
          (`GameplayStatics.SetGamePaused` true)
          (elif (== (`self.Seconds`) 240)
            (`GameplayStatics.OpenLevel` "Level_Main")
            (else
              (`/Engine/EditorBlueprintResources/StandardMacros.IncrementInt` (`self.Seconds`)))))))))

(fn `Next Floor Tile`
  (`parent.Next Floor Tile`)
  (if (== (mod (`self.Current Tile Count`) 3) 1)
    (if (`self.Passed PopUp2`)
      (`self.Add Floor Tile` "NewEnumerator1")
      (else
        (`self.Add Floor Tile` "NewEnumerator0" :!label _label)))
    (else
      (goto _label))))

(fn `UserConstructionScript`
  (`parent.UserConstructionScript`))