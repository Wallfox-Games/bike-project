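; Player controller for the bike game that creates and drives the main, health bar, boss and level-fade HUD widgets.
; Tick blocks movement during the level fade and shows a pause state when pedalling power stays low past a delay.
; Hits trigger a timed invincibility window, and hits and health gains briefly show the health bar and a material-collection flash.
; Movement state changes toggle the boss HUD and its power display.
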(event `self.ReceiveBeginPlay`
  (`parent.ReceiveBeginPlay`)
  (`|ExecutionSequence`
    (:`then_0`
      (bind _returnvalue (`|CreateWidget` "/Game/UserInterface/HUD/HUDWidget.HUDWidget_C" self))
      (bind _output_get (set `self.HUD Reference` _returnvalue))
      (`UserWidget.AddToViewport` _output_get 0))
    (:`then_1`
      (bind _returnvalue_2 (`|CreateWidget` "/Game/UserInterface/HUD/HUDHealthBar.HUDHealthBar_C" self))
      (bind _output_get_2 (set `self.Health Reference` _returnvalue_2))
      (`UserWidget.AddToViewport` _output_get_2 0)
      (`Widget.SetVisibility` _output_get_2 "Collapsed"))
    (:`then_2`
      (bind _returnvalue_3 (`|CreateWidget` "/Game/UserInterface/HUD/HUDBoss.HUDBoss_C" self))
      (bind _output_get_3 (set `self.Boss Reference` _returnvalue_3))
      (`UserWidget.AddToViewport` _output_get_3 0)
      (`Widget.SetVisibility` _output_get_3 "Collapsed"))
    (:`then_3`
      (bind _returnvalue_4 (`|CreateWidget` "/Game/UserInterface/HUD/HUDLevel.HUDLevel_C"))
      (bind _output_get_4 (set `self.Level Widget Reference` _returnvalue_4))
      (`UserWidget.AddToViewport` _output_get_4 0)
      (`/Game/UserInterface/HUD/HUDLevel.Start Fade` _output_get_4 true))))

(event `self.ReceiveTick`
  (params (DeltaSeconds :type "Float (single-precision)"))
  (bind _hud_reference (`self.HUD Reference`))
  (bind _level_widget_reference (`self.Level Widget Reference`))
  (`parent.ReceiveTick` DeltaSeconds)
  (if (not (`UserWidget.IsAnimationPlaying` _level_widget_reference (`/Game/UserInterface/HUD/HUDLevel.Fade` _level_widget_reference)))
    (bind _visible (`/Game/UserInterface/HUD/HUDLevel.Is Begin Play Visible` _level_widget_reference))
    (if _visible
      (if (>= (`self.GetPowerLevel`) 0.1)
        (`/Game/UserInterface/HUD/HUDLevel.Hide Begin Play` _level_widget_reference)
        (if (`self.GetMoveUIBlocked`) :!label _label
          _
          (elif (< (`self.GetPowerLevel`) 0.1)
            (bind _output_get (set `self.PauseDelay` (+ (`self.PauseDelay`) DeltaSeconds)))
            (bind _returnvalue (>= _output_get (`self.Max Pause Delay`)))
            (`self.SetMovePauseBlocked` _returnvalue)
            (`/Game/UserInterface/HUD/HUDWidget.ChangePausedVisibility` _hud_reference _returnvalue)
            (else
              (set `self.PauseDelay` 0.0)
              (`self.SetMovePauseBlocked` false)
              (`/Game/UserInterface/HUD/HUDWidget.ChangePausedVisibility` _hud_reference false)
              (set `self.HealthDelay` (`KismetMathLibrary.FClamp` (- (`self.HealthDelay`) DeltaSeconds) 0.0 (`self.Max Health Delay`)))))))
      (else
        (goto _label)))
    (else
      (`self.SetMovePauseBlocked` true))))

(event `self.PlayerHit`
  (params (OffScreen :type Boolean))
  (bind _health_reference (`self.Health Reference`))
  (if (== (`self.HealthDelay`) 0.0)
    (set `self.HealthDelay` (`self.Max Health Delay`))
    (`parent.PlayerHit` OffScreen)
    (set `/Game/UserInterface/HUD/HUDHealthBar.OffScreen` OffScreen _health_reference)
    (`Widget.SetVisibility` _health_reference "Visible")
    (`KismetMaterialLibrary.SetScalarParameterValue` "/Game/Materials/Material_Functions/MainParameterCollection.MainParameterCollection" "InvincibilityFlash" 1.0)
    (`KismetSystemLibrary.Delay` (`self.Max Health Delay`))
    (`Widget.SetVisibility` _health_reference "Collapsed")
    (`KismetMaterialLibrary.SetScalarParameterValue` "/Game/Materials/Material_Functions/MainParameterCollection.MainParameterCollection" "InvincibilityFlash")))

(event `self.SetMoveEnum`
  (params (NewState :type "EPlayerMove Enum" :default "PME_Normal") (DeltaTime :type "Float (single-precision)"))
  (bind _hud_reference (`self.HUD Reference`))
  (bind _boss_reference (`self.Boss Reference`))
  (`parent.SetMoveEnum` NewState DeltaTime)
  (switch `EPlayerMove` NewState
    (:`PME_Normal`
      (`Widget.SetVisibility` _boss_reference "Collapsed" :!label _label_2)
      (set `/Game/UserInterface/HUD/HUDWidget.Boss InPlay` false _hud_reference))
    (:`PME_BossCharge`
      (`/Game/UserInterface/HUD/HUDBoss.Set Power Visibilty` _boss_reference 1)
      (`Widget.SetVisibility` _boss_reference "Visible" :!label _label_3)
      (set `/Game/UserInterface/HUD/HUDWidget.Boss InPlay` true _hud_reference))
    (:`PME_BossDodge`
      (`/Game/UserInterface/HUD/HUDBoss.Set Power Visibilty` _boss_reference 2)
      (goto _label_3))
    (:`PME_BossAttack`
      (`/Game/UserInterface/HUD/HUDBoss.Set Power Visibilty` _boss_reference 0 :!label _label_4)
      (goto _label_3))
    (:`PME_BossCooldown`
      (goto _label_4))
    (:`PME_SlowDown`
      (goto _label_2))))

(event `self.IncPlayerHealth`
  (params (MaxHealth :type Boolean))
  (bind _health_reference (`self.Health Reference`))
  (`parent.IncPlayerHealth` MaxHealth)
  (set `/Game/UserInterface/HUD/HUDHealthBar.OffScreen` false _health_reference)
  (`Widget.SetVisibility` _health_reference "Visible")
  (`KismetMaterialLibrary.SetScalarParameterValue` "/Game/Materials/Material_Functions/MainParameterCollection.MainParameterCollection" "InvincibilityFlash" 1.0)
  (`KismetSystemLibrary.Delay` 1.0)
  (`Widget.SetVisibility` _health_reference "Collapsed")
  (`KismetMaterialLibrary.SetScalarParameterValue` "/Game/Materials/Material_Functions/MainParameterCollection.MainParameterCollection" "InvincibilityFlash"))

(fn `UserConstructionScript`)