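; Player character Blueprint for a bike game, handling hit reactions and lane-blocked feedback.
; Tick stores the Location component's transform as SpawnLocation and polls a Hit flag on BikeGameInstance, clearing it and calling BeenHit.
; BeenHit decrements game-instance health, zeroes the multiplier and briefly shows the PlayerHealth display.
; SetLaneBlocked calls the parent, then toggles the blocked indicator on the HUD cached from BP_BikePlayerController.
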(event `self.ReceiveBeginPlay`
  (bind _asbp_bike_player_controller (cast `/Game/Blueprints/Player/BP_BikePlayerController` (`GameplayStatics.GetPlayerController` 0)))
  (set `self.HUD Reference` (`/Game/Blueprints/Player/BP_BikePlayerController.HUD Reference` _asbp_bike_player_controller)))

(event `self.ReceiveTick`
  (params (DeltaSeconds :type "Float (single-precision)"))
  (set `self.Spawn Location` (`SceneComponent.K2_GetComponentToWorld` (`self.location`)))
  (bind _asbike_game_instance (cast `BikeGameInstance` (`GameplayStatics.GetGameInstance`)))
  (if (`BikeGameInstance.GetHit` _asbike_game_instance)
    (`BikeGameInstance.SetHit` _asbike_game_instance false)
    (`self.BeenHit`)))

(event `BeenHit`
  ;[1 1 1] Function for when the player is hit
  (`SceneComponent.SetVisibility` (`self.Player Health`) true false)
  (bind _asbike_game_instance (cast `BikeGameInstance` (`GameplayStatics.GetGameInstance`)))
  (bind _result (`/Engine/EditorBlueprintResources/StandardMacros.DecrementInt` (`BikeGameInstance.PlayerHealth` _asbike_game_instance))
    (:`  `
      (`BikeGameInstance.SetPlayerHealth` _asbike_game_instance _result)
      (`BikeGameInstance.SetMultiplier` _asbike_game_instance 0)
      (`KismetSystemLibrary.Delay` 2.0)
      (`SceneComponent.SetVisibility` (`self.Player Health`) false false))))

(event `Return Sapwn Location`)

(event `self.SetLaneBlocked`
  (params (Blocking :type Boolean))
  (`parent.SetLaneBlocked` Blocking)
  (`/Game/UserInterface/HUD.ChangeBlockedVisibility` (`self.HUD Reference`) Blocking))

(fn `UserConstructionScript`)