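; Floor-tile runner controller, apparently a timed tutorial or calibration stage, that seeds ten tiles and shows four timed pop-ups.
; Tick uses a one-second Delay to count Seconds, pausing at each pop-up threshold; those branches never increment the counter.
; NextFloorTile swaps every third tile to another type once PassedPopUp2 is set.
; Logic saving steady player power as max power before loading Level_Main is disconnected.
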(event `self.ReceiveBeginPlay`
  (`parent.ReceiveBeginPlay`)
  (set `self.Current Power` 0.0)
  (set `self.Passed PopUp2` false)
  (set `self.Current Tile Count` 0)
  (for _ (range 10)
    (`self.Next Floor Tile`)))

(event `self.ReceiveTick`
  (params (DeltaSeconds :type "Float (single-precision)"))
  (`KismetSystemLibrary.Delay` 1.0)
  (if (== (`self.Seconds`) 45)
    (bind _returnvalue (`|CreateWidget` "/Game/Blueprints/PopUp1.PopUp1_C"))
    (`UserWidget.AddToViewport` _returnvalue 0)
    (`GameplayStatics.SetGamePaused` true)
    (`KismetSystemLibrary.Delay` 10.0)
    (`GameplayStatics.SetGamePaused` false)
    (elif (== (`self.Seconds`) 90)
      (bind _returnvalue_2 (`|CreateWidget` "/Game/Blueprints/PopUp2.PopUp2_C"))
      (`UserWidget.AddToViewport` _returnvalue_2 0)
      (`GameplayStatics.SetGamePaused` true)
      (`KismetSystemLibrary.Delay` 10.0)
      (set `self.Passed PopUp2` true)
      (`GameplayStatics.SetGamePaused` false)
      (elif (== (`self.Seconds`) 135)
        (bind _returnvalue_3 (`|CreateWidget` "/Game/Blueprints/PopUp3.PopUp3_C"))
        (`UserWidget.AddToViewport` _returnvalue_3 0)
        (`GameplayStatics.SetGamePaused` true)
        (`KismetSystemLibrary.Delay` 10.0)
        (`GameplayStatics.SetGamePaused` false)
        (elif (== (`self.Seconds`) 180)
          (bind _returnvalue_4 (`|CreateWidget` "/Game/Blueprints/PopUp4.PopUp4_C"))
          (`UserWidget.AddToViewport` _returnvalue_4 0)
          (`GameplayStatics.SetGamePaused` true)
          (`KismetSystemLibrary.Delay` 10.0)
          (`GameplayStatics.SetGamePaused` false)
          (elif (not (== (`self.Seconds`) 240))
            (`/Engine/EditorBlueprintResources/StandardMacros.IncrementInt` (`self.Seconds`))))))))

(fn `Next Floor Tile`
  (`parent.Next Floor Tile`)
  (if (== (mod (`self.Current Tile Count`) 3) 1)
    (if (`self.Passed PopUp2`)
      (`self.Add Floor Tile` "NewEnumerator1")
      (else
        (`self.Add Floor Tile` "NewEnumerator0" :!label _label)))
    (else
      (goto _label))))

(fn `UserConstructionScript`
  (`parent.UserConstructionScript`))