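; Test Blueprint that procedurally builds an angled road bend tile with raised brick edging in its Construction Script; its event graph is unused.
; Trigonometry on Angle, TileSize and RoadSections shapes the MainRoadProcedural corner mesh, with plane meshes added as straight entry and exit pieces.
; The corner is computed from the absolute angle and mirrored by negative X scale for negative bends.
; BricksOuter derives its edging from the same corner points plus brick offset, width and height.
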(fn `UserConstructionScript`
  (bind _bricks_offset (`self.Bricks Offset`))
  (bind _bricks_offset_2 (`self.Bricks Offset`))
  (bind _angle (`self.Angle`))
  (bind _brick_width (`self.Brick Width`))
  (bind _bricks_inner_ (`self.Bricks(Inner)`))
  (bind _brick_height (`self.Brick Height`))
  (bind _brick_height_2 (`self.Brick Height`))
  (bind _brick_width_2 (`self.Brick Width`))
  (bind _mainroadprocedural (`self.MainRoadProcedural`))
  (bind _axis (`self.Axis`))
  (bind (_x _y) (`KismetMathLibrary.BreakVector2D` (`self.UV Tiling Brick`)))
  (bind _returnvalue (- (`self.Brick Height`) 1.41))
  (bind _returnvalue_2 (- (`self.Brick Height`) 1.41))
  (bind _returnvalue_3 (`KismetMathLibrary.Abs` (`self.Angle`)))
  (bind _returnvalue_4 (`KismetMathLibrary.Abs` _angle))
  (bind _returnvalue_5 (/ (`self.Tile Size`) (`KismetMathLibrary.Conv_IntToDouble` (`self.Road Sections`))))
  (bind _returnvalue_6 (- (`KismetMathLibrary.Abs` (`self.Angle`)) 45.0))
  (bind _returnvalue_7 (/ _x 2.0))
  (bind _returnvalue_8 (/ (`self.Tile Size`) (`KismetMathLibrary.Conv_IntToDouble` (`self.Road Sections`))))
  (bind _returnvalue_9 (- (`KismetMathLibrary.Abs` (`self.Angle`)) 135.0))
  (bind _returnvalue_10 (- 90.0 _returnvalue_3))
  (bind _returnvalue_11 (/ (`self.Tile Size`) (`KismetMathLibrary.Conv_IntToDouble` (`self.Road Sections`))))
  (bind _returnvalue_12 (* _y (/ (`self.Brick Height`) 100.0)))
  (bind _returnvalue_13 (`KismetMathLibrary.MakeVector` _returnvalue_11 _returnvalue_11 _returnvalue_11))
  (bind _returnvalue_14 (* (/ (`self.Tile Size`) (`KismetMathLibrary.Conv_IntToDouble` (`self.Road Sections`))) 100.0))
  (bind _returnvalue_15 (* _returnvalue_8 300.0))
  (bind _returnvalue_16 (* _returnvalue_8 50.0))
  (bind _returnvalue_17 (/ _returnvalue_14 2.0))
  (bind _returnvalue_18 (/ _returnvalue_14 2.0))
  (bind _returnvalue_19 (- _returnvalue_16 _bricks_offset))
  (bind _returnvalue_20 (`KismetMathLibrary.Square` _returnvalue_16))
  (bind _returnvalue_21 (* _returnvalue_14 1.5))
  (bind _returnvalue_22 (- (+ _returnvalue_16 (* (`self.Brick Width`) _returnvalue_8)) _bricks_offset))
  (bind _returnvalue_23 (* _returnvalue_18 -1.0))
  (bind _returnvalue_24 (+ _returnvalue_12 (/ (* (/ (`self.Tile Size`) (`KismetMathLibrary.Conv_IntToDouble` (`self.Road Sections`))) (`self.Brick Width`)) 200.0)))
  (bind _returnvalue_25 (* _returnvalue_19 -1.0))
  (bind _returnvalue_26 (`KismetMathLibrary.MakeVector` _returnvalue_22 0.0 _returnvalue_2))
  (bind _returnvalue_27 (`KismetMathLibrary.Sqrt` (+ _returnvalue_20 _returnvalue_20)))
  (bind _returnvalue_28 (`KismetMathLibrary.MakeVector` (- (.x (0.0 0.0 0.0)) _returnvalue_17) (+ (.y (0.0 0.0 0.0)) _returnvalue_21) (.z (0.0 0.0 0.0))))
  (bind _returnvalue_29 (+ (* (+ (* _returnvalue_5 50.0) (* _brick_width_2 _returnvalue_5)) -1.0) (`self.Bricks Offset`)))
  (bind _returnvalue_30 (+ _returnvalue_24 (/ 1.41 100.0)))
  (bind _returnvalue_31 (+ _returnvalue_24 (/ 1.41 100.0)))
  (bind _returnvalue_32 (* (/ (+ _returnvalue_15 (* (`KismetMathLibrary.DegTan` (/ (`KismetMathLibrary.Abs` (`self.Angle`)) 2.0)) (* _returnvalue_8 100.0))) _returnvalue_15) _x))
  (bind _returnvalue_33 (/ _returnvalue_32 2.0))
  (bind _returnvalue_34 (`KismetMathLibrary.MakeVector` (- (.x (`KismetMathLibrary.MakeVector` _returnvalue_14 (* (`KismetMathLibrary.DegTan` (/ _returnvalue_4 2.0)) _returnvalue_14))) _returnvalue_17) (+ (.y (`KismetMathLibrary.MakeVector` _returnvalue_14 (* (`KismetMathLibrary.DegTan` (/ _returnvalue_4 2.0)) _returnvalue_14))) _returnvalue_21) (.z (`KismetMathLibrary.MakeVector` _returnvalue_14 (* (`KismetMathLibrary.DegTan` (/ _returnvalue_4 2.0)) _returnvalue_14)))))
  (bind _returnvalue_35 (- (.x (`KismetMathLibrary.RotateAngleAxis` (`KismetMathLibrary.MakeVector` _returnvalue_14 _returnvalue_18) _returnvalue_4 _axis)) _returnvalue_17))
  (bind _returnvalue_36 (- (.x (`KismetMathLibrary.RotateAngleAxis` (`KismetMathLibrary.MakeVector` 0.0 _returnvalue_18) _returnvalue_4 _axis)) _returnvalue_17))
  (bind _returnvalue_37 (+ (.y (`KismetMathLibrary.RotateAngleAxis` (`KismetMathLibrary.MakeVector` _returnvalue_14 _returnvalue_18) _returnvalue_4 _axis)) _returnvalue_21))
  (bind _returnvalue_38 (+ (.y (`KismetMathLibrary.RotateAngleAxis` (`KismetMathLibrary.MakeVector` 0.0 _returnvalue_18) _returnvalue_4 _axis)) _returnvalue_21))
  (bind _returnvalue_39 (`KismetMathLibrary.MakeVector` _returnvalue_36 _returnvalue_38 (.z (`KismetMathLibrary.RotateAngleAxis` (`KismetMathLibrary.MakeVector` 0.0 _returnvalue_18) _returnvalue_4 _axis))))
  (bind _returnvalue_40 (`KismetMathLibrary.MakeVector` _returnvalue_35 _returnvalue_37 (.z (`KismetMathLibrary.RotateAngleAxis` (`KismetMathLibrary.MakeVector` _returnvalue_14 _returnvalue_18) _returnvalue_4 _axis))))
  (bind _returnvalue_41 (`KismetMathLibrary.Normal` (- _returnvalue_34 _returnvalue_28)))
  (bind _x_2 (.x _returnvalue_41))
  (bind _y_2 (.y _returnvalue_41))
  (bind _x_3 (.x (`KismetMathLibrary.Normal` (- _returnvalue_40 _returnvalue_39))))
  (bind _y_3 (.y (`KismetMathLibrary.Normal` (- _returnvalue_40 _returnvalue_39))))
  (bind _returnvalue_42 (* _bricks_offset (.x (* _returnvalue_41 -1.0))))
  (bind _returnvalue_43 (* (.y (* _returnvalue_41 -1.0)) _bricks_offset))
  (bind _returnvalue_44 (* _y_3 _bricks_offset_2))
  (bind _returnvalue_45 (* _x_3 _bricks_offset_2))
  (bind _returnvalue_46 (- (.x _returnvalue_28) _returnvalue_42))
  (bind _returnvalue_47 (- (.y _returnvalue_28) _returnvalue_43))
  (bind _returnvalue_48 (`KismetMathLibrary.MakeVector` (- (- (+ (/ (+ _returnvalue_36 _returnvalue_35) 2.0) (* (`KismetMathLibrary.DegCos` _returnvalue_3) _returnvalue_18)) (/ (- _returnvalue_35 _returnvalue_36) 2.0)) (* (`KismetMathLibrary.DegCos` _returnvalue_10) _returnvalue_18)) (+ (* _returnvalue_18 (`KismetMathLibrary.DegSin` _returnvalue_10)) (- (+ (/ (+ _returnvalue_38 _returnvalue_37) 2.0) (* (`KismetMathLibrary.DegSin` _returnvalue_3) _returnvalue_18)) (/ (- _returnvalue_37 _returnvalue_38) 2.0)))))
  (bind _returnvalue_49 (- _returnvalue_46 (* _brick_width_2 _returnvalue_5 _x_2)))
  (bind _returnvalue_50 (- _returnvalue_47 (* _brick_width_2 _returnvalue_5 _y_2)))
  (bind _x_4 (.x _returnvalue_48))
  (bind _y_4 (.y _returnvalue_48))
  (bind _returnvalue_51 (`KismetMathLibrary.MakeVector` (+ (.x _returnvalue_34) _returnvalue_42) (+ (.y _returnvalue_34) _returnvalue_43) (.z _returnvalue_34)))
  (bind _x_5 (.x _returnvalue_51))
  (bind _y_5 (.y _returnvalue_51))
  (bind _returnvalue_52 (- (- _x_4 (* (`KismetMathLibrary.DegCos` _returnvalue_9) _returnvalue_27)) _returnvalue_45))
  (bind _returnvalue_53 (- (- _y_4 (* (`KismetMathLibrary.DegSin` _returnvalue_9) _returnvalue_27)) _returnvalue_44))
  (bind _returnvalue_54 (+ (- _x_4 (* (`KismetMathLibrary.DegCos` _returnvalue_6) _returnvalue_27)) _returnvalue_45))
  (bind _returnvalue_55 (+ _x_5 (* _brick_width _returnvalue_8 _x_2)))
  (bind _returnvalue_56 (+ _y_5 (* _brick_width _returnvalue_8 _y_2)))
  (bind _returnvalue_57 (+ (- _y_4 (* (`KismetMathLibrary.DegSin` _returnvalue_6) _returnvalue_27)) _returnvalue_44))
  (bind _returnvalue_58 (- _returnvalue_57 (* _returnvalue_5 _brick_width_2 _y_3)))
  (bind _returnvalue_59 (- _returnvalue_54 (* _returnvalue_5 _brick_width_2 _x_3)))
  (bind _returnvalue_60 (`KismetMathLibrary.MakeVector` _returnvalue_55 _returnvalue_56 _returnvalue_2))
  (bind _returnvalue_61 (+ _returnvalue_53 (* _brick_width _returnvalue_8 _y_3)))
  (bind _returnvalue_62 (+ _returnvalue_52 (* _brick_width _returnvalue_8 _x_3)))
  (bind _returnvalue_63 (`KismetMathLibrary.MakeVector` _returnvalue_62 _returnvalue_61 _returnvalue_2))
  (`ProceduralMeshComponent.CreateMeshSection_LinearColor` :`self` (`self.MainRoadProcedural`) :`Vertices` (`|MakeArray` (`KismetMathLibrary.MakeVector` (- (.x (`KismetMathLibrary.MakeVector` 0.0 _returnvalue_23)) _returnvalue_17) (+ (.y (`KismetMathLibrary.MakeVector` 0.0 _returnvalue_23)) _returnvalue_21) (.z (`KismetMathLibrary.MakeVector` 0.0 _returnvalue_23))) (`KismetMathLibrary.MakeVector` (- (.x (`KismetMathLibrary.MakeVector` _returnvalue_14 _returnvalue_23)) _returnvalue_17) (+ (.y (`KismetMathLibrary.MakeVector` _returnvalue_14 _returnvalue_23)) _returnvalue_21) (.z (`KismetMathLibrary.MakeVector` _returnvalue_14 _returnvalue_23))) _returnvalue_28 _returnvalue_34 _returnvalue_39 _returnvalue_40) :`Triangles` (`|MakeArray` 1 0 2 3 1 2 3 2 4 3 4 5) :`UV0` (`|MakeArray` (0.0 0.0) (1.0 0.0) (0.0 0.5) (1.0 0.5) (0.0 1.0) (1.0 1.0) :!type "Vector2D Structure"))
  (`PrimitiveComponent.SetMaterial` (`self.MainRoadProcedural`) 0 "/Game/Materials/Tileables/M_Tileable_Road.M_Tileable_Road")
  (if (< _angle 0.0)
    (`SceneComponent.SetRelativeScale3D` _mainroadprocedural (-1.0 1.0 1.0))
    (bind _returnvalue_64 (`AddComponent|NODE_AddStaticMeshComponent-1` :`RelativeTransform` (`KismetMathLibrary.MakeTransform` _returnvalue_48 (`KismetMathLibrary.MakeRotator` 0.0 0.0 (* (`self.Angle`) -1.0)) _returnvalue_13)))
    (`StaticMeshComponent.SetStaticMesh` _returnvalue_64 "/Game/Meshes/Shapes/Shape_Plane.Shape_Plane")
    (`PrimitiveComponent.SetMaterial` _returnvalue_64 0 "/Game/Materials/Tileables/M_Tileable_Road.M_Tileable_Road")
    (else
      (`SceneComponent.SetRelativeScale3D` _mainroadprocedural (1.0 1.0 1.0))
      (bind _returnvalue_65 (`AddComponent|NODE_AddStaticMeshComponent-2` :`RelativeTransform` (`KismetMathLibrary.MakeTransform` _returnvalue_48 (`KismetMathLibrary.MakeRotator` 0.0 0.0 (`self.Angle`)) _returnvalue_13)))
      (`StaticMeshComponent.SetStaticMesh` _returnvalue_65 "/Game/Meshes/Shapes/Shape_Plane.Shape_Plane")
      (`PrimitiveComponent.SetMaterial` _returnvalue_65 0 "/Game/Materials/Tileables/M_Tileable_Road.M_Tileable_Road")))
  (bind _returnvalue_66 (`AddComponent|NODE_AddStaticMeshComponent-3` :`RelativeTransform` (`KismetMathLibrary.MakeTransform` (`KismetMathLibrary.MakeVector` 0.0 (* _returnvalue_11 50.0)) (struct) _returnvalue_13)))
  (`StaticMeshComponent.SetStaticMesh` _returnvalue_66 "/Game/Meshes/Shapes/Shape_Plane.Shape_Plane")
  (`PrimitiveComponent.SetMaterial` _returnvalue_66 0 "/Game/Materials/Tileables/M_Tileable_Road.M_Tileable_Road")
  (`ProceduralMeshComponent.CreateMeshSection_LinearColor` :`self` (`self.Bricks(Outer)`) :`Vertices` (`|MakeArray` (`KismetMathLibrary.MakeVector` _returnvalue_19) _returnvalue_51 (`KismetMathLibrary.MakeVector` _returnvalue_52 _returnvalue_53) (`KismetMathLibrary.MakeVector` _returnvalue_19 0.0 _brick_height_2) (`KismetMathLibrary.MakeVector` _x_5 _y_5 _brick_height_2) (`KismetMathLibrary.MakeVector` _returnvalue_52 _returnvalue_53 _brick_height_2) (`KismetMathLibrary.MakeVector` _returnvalue_22 0.0 _brick_height_2) (`KismetMathLibrary.MakeVector` _returnvalue_55 _returnvalue_56 _brick_height_2) (`KismetMathLibrary.MakeVector` _returnvalue_62 _returnvalue_61 _brick_height_2) _returnvalue_26 _returnvalue_60 _returnvalue_63) :`Triangles` (`|MakeArray` 0 1 3 1 4 3 1 2 4 2 5 4 3 4 6 4 7 6 4 5 7 7 5 8 6 7 9 9 7 10 7 8 10 8 11 10) :`UV0` (`|MakeArray` (`KismetMathLibrary.MakeVector2D` 0.0) (`KismetMathLibrary.MakeVector2D` _returnvalue_33) (`KismetMathLibrary.MakeVector2D` _returnvalue_32) (`KismetMathLibrary.MakeVector2D` 0.0 _returnvalue_12) (`KismetMathLibrary.MakeVector2D` _returnvalue_33 _returnvalue_12) (`KismetMathLibrary.MakeVector2D` _returnvalue_32 _returnvalue_12) (`KismetMathLibrary.MakeVector2D` 0.0 _returnvalue_24) (`KismetMathLibrary.MakeVector2D` _returnvalue_33 _returnvalue_24) (`KismetMathLibrary.MakeVector2D` _returnvalue_32 _returnvalue_24) (`KismetMathLibrary.MakeVector2D` 0.0 _returnvalue_30) (`KismetMathLibrary.MakeVector2D` _returnvalue_33 _returnvalue_30) (`KismetMathLibrary.MakeVector2D` _returnvalue_32 _returnvalue_30)))
  (`PrimitiveComponent.SetMaterial` (`self.Bricks(Outer)`) 0 "/Game/Materials/Trims/M_Trim_01.M_Trim_01")
  (`ProceduralMeshComponent.CreateMeshSection_LinearColor` :`self` _bricks_inner_ :`Vertices` (`|MakeArray` (`KismetMathLibrary.MakeVector` _returnvalue_25) (`KismetMathLibrary.MakeVector` _returnvalue_46 _returnvalue_47 (.z _returnvalue_28)) (`KismetMathLibrary.MakeVector` _returnvalue_54 _returnvalue_57) (`KismetMathLibrary.MakeVector` _returnvalue_25 0.0 _brick_height) (`KismetMathLibrary.MakeVector` _returnvalue_46 _returnvalue_47 _brick_height) (`KismetMathLibrary.MakeVector` _returnvalue_54 _returnvalue_57 _brick_height) (`KismetMathLibrary.MakeVector` _returnvalue_29 0.0 _brick_height) (`KismetMathLibrary.MakeVector` _returnvalue_49 _returnvalue_50 _brick_height) (`KismetMathLibrary.MakeVector` _returnvalue_59 _returnvalue_58 _brick_height) (`KismetMathLibrary.MakeVector` _returnvalue_29 0.0 _returnvalue) (`KismetMathLibrary.MakeVector` _returnvalue_49 _returnvalue_50 _returnvalue) (`KismetMathLibrary.MakeVector` _returnvalue_59 _returnvalue_58 _returnvalue)) :`Triangles` (`|MakeArray` 3 1 0 3 4 1 4 2 1 2 4 5 6 4 3 6 7 4 4 7 8 5 4 8 9 7 6 10 7 9 7 10 8 11 8 10) :`UV0` (`|MakeArray` (`KismetMathLibrary.MakeVector2D` 0.0) (`KismetMathLibrary.MakeVector2D` _returnvalue_7 0.0) (`KismetMathLibrary.MakeVector2D` _x) (`KismetMathLibrary.MakeVector2D` 0.0 _returnvalue_12) (`KismetMathLibrary.MakeVector2D` _returnvalue_7 _returnvalue_12) (`KismetMathLibrary.MakeVector2D` _x _returnvalue_12) (`KismetMathLibrary.MakeVector2D` 0.0 _returnvalue_24) (`KismetMathLibrary.MakeVector2D` _returnvalue_7 _returnvalue_24) (`KismetMathLibrary.MakeVector2D` _x _returnvalue_24) (`KismetMathLibrary.MakeVector2D` 0.0 _returnvalue_31) (`KismetMathLibrary.MakeVector2D` _returnvalue_7 _returnvalue_31) (`KismetMathLibrary.MakeVector2D` _x _returnvalue_31)))
  (`PrimitiveComponent.SetMaterial` _bricks_inner_ 0 "/Game/Materials/Trims/M_Trim_01.M_Trim_01")
  (`ProceduralMeshComponent.CreateMeshSection_LinearColor` :`self` (`self.Pavement(Outer)`) :`Vertices` (`|MakeArray` _returnvalue_26 _returnvalue_60 _returnvalue_63 (0.0 0.0 0.0) (0.0 0.0 0.0) (0.0 0.0 0.0)) :`Triangles` (`|MakeArray` 0) :`UV0` (`|MakeArray` (0.0 0.0) :!type "Vector2D Structure")))