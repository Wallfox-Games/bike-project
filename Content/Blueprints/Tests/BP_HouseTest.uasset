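; BP_HouseTest is a test actor that generates a randomly sized building from a single mesh.
; Its Construction Script adds a static mesh component at the actor origin, scales each axis independently within its Min/Max variables, and assigns BuildingMesh.
; The random scale is unseeded, so the size re-rolls whenever construction reruns.
; The event graph holds only disabled placeholder events.
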(fn `UserConstructionScript`
  (bind _returnvalue (`AddComponent|NODE_AddStaticMeshComponent-0` :`RelativeTransform` (`KismetMathLibrary.MakeTransform` (0.0 0.0 0.0) (struct) (`KismetMathLibrary.MakeVector` (`KismetMathLibrary.RandomFloatInRange` (`self.MinX`) (`self.MaxX`)) (`KismetMathLibrary.RandomFloatInRange` (`self.MinY`) (`self.MaxY`)) (`KismetMathLibrary.RandomFloatInRange` (`self.MinZ`) (`self.MaxZ`))))))
  (`StaticMeshComponent.SetStaticMesh` _returnvalue (`self.BuildingMesh`)))