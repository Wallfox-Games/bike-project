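; Test city tile that procedurally builds a floor and rows of multi-storey buildings along its Y sides in the Construction Script.
; It creates per-colour HISM components for ground and upper floors, tinted from BP_LevelDatabaseActor's palette.
; A grid of downward traces places seeded random stacks, mirroring Y for the opposite side.
; Box tests cut gaps for crossroads and T-junctions, and the tile rotates in quarter turns.
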(fn `Building Placement`
  (params (`In Hit (LineTrace)` :type "HitResult Structure") (`Ground Floor Mesh` :type "InstancedStaticMeshComponent Object Reference") (`Floor Mesh` :type "InstancedStaticMeshComponent Object Reference") (`Building Spawn Y Direction` :type "Float (double-precision)" :default 1.0) (`Rotation (Yaw)` :type "Float (double-precision)" :default -90.0) (`Current Point` :type Integer))
  (bind _returnvalue (`KismetMathLibrary.MakeRotator` 0.0 0.0 `Rotation (Yaw)`))
  (bind (_bblockinghit _binitialoverlap _time _distance _location _impactpoint) (`GameplayStatics.BreakHitResult` `In Hit (LineTrace)`))
  (bind (_min _max) (`StaticMeshComponent.GetLocalBounds` `Ground Floor Mesh`))
  (bind _max_floors (`self.Max Floors`))
  (bind _building_scale (`self.Building Scale`))
  (bind _building_scale_2 (`self.Building Scale`))
  (bind _building_scale_3 (`self.Building Scale`))
  (bind _returnvalue_2 (`KismetMathLibrary.RandomIntegerInRangeFromStream` (`self.Min Floors`) _max_floors (`self.Seed`)))
  (bind _z (.z (* _max _building_scale_3)))
  (bind _returnvalue_3 (`KismetMathLibrary.MakeVector` (.x (- _impactpoint (`self.K2_GetActorLocation`))) (* (.y (- _impactpoint (`self.K2_GetActorLocation`))) `Building Spawn Y Direction`) _z))
  (if _bblockinghit
    (`InstancedStaticMeshComponent.AddInstance` `Ground Floor Mesh` (`KismetMathLibrary.MakeTransform` _returnvalue_3 _returnvalue (`KismetMathLibrary.MakeVector` _building_scale _building_scale _building_scale)))
    (bind _returnvalue_4 (`PrimitiveComponent.CreateDynamicMaterialInstance` `Ground Floor Mesh` (`MeshComponent.GetMaterialIndex` `Ground Floor Mesh` "Building_Front") "/Game/Materials/Master_Materials/MM_Building_Front.MM_Building_Front" "None"))
    (`MaterialInstanceDynamic.SetScalarParameterValue` _returnvalue_4 "UseRandSlot" 1.0)
    (`MaterialInstanceDynamic.SetScalarParameterValue` _returnvalue_4 "Random_Per_Building" 4.0)
    (`MaterialInstanceDynamic.SetScalarParameterValue` _returnvalue_4 "SecondRand" 13.0)
    (switch `int` _max_floors
      (:`Default`
        (for _index (range _returnvalue_2)
          (switch `int` _returnvalue_2
            (:`Default`
              (`InstancedStaticMeshComponent.AddInstance` `Floor Mesh` (`KismetMathLibrary.MakeTransform` (`KismetMathLibrary.MakeVector` (.x _returnvalue_3) (.y _returnvalue_3) (+ (* (.z _returnvalue_3) 3.0) (* _index (- _z (.z (* _min _building_scale_3)))))) _returnvalue (`KismetMathLibrary.MakeVector` _building_scale_2 _building_scale_2 _building_scale_2))))
            (:`0`
              (return)))))
      (:`0`
        _))
    (return)))

(fn `UserConstructionScript`
  (bind _tile_size (`self.Tile Size`))
  (bind _tile_size_2 (`self.Tile Size`))
  (bind _tile_size_3 (`self.Tile Size`))
  (bind _returnvalue (/ _tile_size_3 2.0))
  (bind _returnvalue_2 (/ _tile_size 2.0))
  (bind _returnvalue_3 (* _tile_size_3 (`self.Spawn Width`)))
  (bind _returnvalue_4 (* _tile_size (`self.Spawn Width`)))
  (bind _returnvalue_5 (- (`KismetArrayLibrary.Array_Length` (`self.Building Base Colour`)) 1))
  (bind _returnvalue_6 (`KismetMathLibrary.MakeVector` _tile_size _returnvalue_4 _tile_size))
  (bind _returnvalue_7 (* _returnvalue_2 100.0))
  (bind _returnvalue_8 (`KismetMathLibrary.RandomIntegerInRangeFromStream` 0 (- (`KismetArrayLibrary.Array_Length` (`self.Bottom Floor Mesh Instances`)) 1) (`self.Seed`)))
  (bind _returnvalue_9 (* (- _returnvalue_2 (/ _returnvalue_4 2.0)) 100.0))
  (bind _output (`|GetArrayItem` (`self.Upper Floor Mesh Instances`) _returnvalue_8))
  (bind _output_2 (`|GetArrayItem` (`self.Bottom Floor Mesh Instances`) _returnvalue_8))
  (bind _returnvalue_10 (`KismetMathLibrary.MakeVector` 0.0 _returnvalue_9 _returnvalue_7))
  ;[0.04116 0.9702 1] Tile Creation
  (bind _returnvalue_11 (`AddComponent|NODE_AddStaticMeshComponent-0` :`RelativeTransform` (`KismetMathLibrary.MakeTransform` (0.0 0.0 0.0) (struct) (`KismetMathLibrary.MakeVector` _tile_size_2 _tile_size_2 _tile_size_2))))
  (`StaticMeshComponent.SetStaticMesh` _returnvalue_11 (`self.FloorMesh`))
  ;[0.02228 1 0.1681] GET Global Variables
  (bind _outactors (`GameplayStatics.GetAllActorsOfClass` "/Game/Blueprints/Tests/BP_LevelDatabaseActor.BP_LevelDatabaseActor_C"))
  (set `self.Building Base Colour` (`/Game/Blueprints/Tests/BP_LevelDatabaseActor.Building Colours` (`|GetArrayItem` _outactors)))
  ;[1 0.4594 0.2061] Spawn Regions
  (`AddComponent|NODE_AddBoxComponent-0` :`RelativeTransform` (`KismetMathLibrary.MakeTransform` _returnvalue_10 (struct) _returnvalue_6))
  (`AddComponent|NODE_AddBoxComponent-1` :`RelativeTransform` (`KismetMathLibrary.MakeTransform` (`KismetMathLibrary.MakeVector` 0.0 (* -1 _returnvalue_9) _returnvalue_7) (struct) _returnvalue_6))
  ;[0.04843 1 0.9203] Set Building Mesh
  (`StaticMeshComponent.SetStaticMesh` (`self.HierarchicalInstancedStaticMesh`) (`self.Building Mesh`))
  (`StaticMeshComponent.SetStaticMesh` (`self.HierarchicalBottomFloorMeshInstance`) (`self.Bottom Floor Mesh`))
  (for _index (range (+ _returnvalue_5 1))
    ;[0.02611 1 0.06393] SET Ground Floor Mesh Array
    (bind _returnvalue_12 (`AddComponent|NODE_AddHierarchicalInstancedStaticMeshComponent-0` :`bManualAttachment` true :`RelativeTransform` (`KismetMathLibrary.MakeTransform` (0.0 0.0 0.0))))
    (`SceneComponent.K2_AttachToComponent` _returnvalue_12 (`self.Scene`) "None" "KeepRelative" "KeepRelative" "KeepRelative" true)
    (`StaticMeshComponent.SetStaticMesh` _returnvalue_12 (`self.Bottom Floor Mesh`))
    (bind _returnvalue_13 (`PrimitiveComponent.CreateDynamicMaterialInstance` _returnvalue_12 0 "/Game/Materials/Placeholders/M_Test_Building_Brick_Inst.M_Test_Building_Brick_Inst" "None"))
    (`MaterialInstanceDynamic.SetVectorParameterValue` _returnvalue_13 "Colour1" (`KismetMathLibrary.Conv_ColorToLinearColor` (`|GetArrayItem` (`self.Building Base Colour`) _index)))
    (`KismetArrayLibrary.Array_Add` (`self.Bottom Floor Mesh Instances`) _returnvalue_12))
  (for _index_2 (range (+ _returnvalue_5 1))
    ;[0.1075 1 0.08636] SET Upper Floor Mesh Array
    (bind _returnvalue_14 (`AddComponent|NODE_AddHierarchicalInstancedStaticMeshComponent-1` :`bManualAttachment` true :`RelativeTransform` (`KismetMathLibrary.MakeTransform` (0.0 0.0 0.0))))
    (`SceneComponent.K2_AttachToComponent` _returnvalue_14 (`self.Scene`) "None" "KeepRelative" "KeepRelative" "KeepRelative" true)
    (`StaticMeshComponent.SetStaticMesh` _returnvalue_14 (`self.Building Mesh`))
    (bind _returnvalue_15 (`PrimitiveComponent.CreateDynamicMaterialInstance` _returnvalue_14 0 "/Game/Materials/Placeholders/M_Test_Building_Brick_Inst.M_Test_Building_Brick_Inst" "None"))
    (`MaterialInstanceDynamic.SetVectorParameterValue` _returnvalue_15 "Colour1" (`KismetMathLibrary.Conv_ColorToLinearColor` (`|GetArrayItem` (`self.Building Base Colour`) _index_2)))
    (`KismetArrayLibrary.Array_Add` (`self.Upper Floor Mesh Instances`) _returnvalue_14))
  ;[1 0.4067 0.1435] Building Spawn Grid
  (bind (_current_point _total_points _0_1_phase _poly_center) (`/Engine/ArtTools/RenderToTexture/Macros/RenderToTextureMacros.2D Grid Execution Macro` (`self.Grid Size (Spacing)`) (+ (`self.K2_GetActorLocation`) _returnvalue_10) (`self.Building Amount (X)`) (`self.Building Amount (Y)`))
    (:`Per Poly Execution`
      (bind _outhit (`KismetSystemLibrary.LineTraceSingle` :`Start` _poly_center :`End` (`KismetMathLibrary.MakeVector` (.x _poly_center) (.y _poly_center) (- (.z _poly_center) (* (`self.Tile Size`) 60.0))) :`TraceChannel` "TraceTypeQuery1" :`bIgnoreSelf` false :`DrawTime` 0.1))
      (if (`self.Crossroad`)
        (bind _returnvalue_16 (`KismetMathLibrary.IsPointInBox` (`.ImpactPoint` (`GameplayStatics.BreakHitResult` _outhit)) (+ (`self.K2_GetActorLocation`) (`KismetMathLibrary.MakeVector` 0.0 (* (- _returnvalue (/ _returnvalue_3 2.0)) 100.0) (* _returnvalue 100.0))) (* (`KismetMathLibrary.MakeVector` (- _tile_size_3 (* _returnvalue_3 2.0)) (/ _tile_size_3 2.0) _tile_size_3) 50.0)))
        (if (not _returnvalue_16)
          ;[0.1309 0.7991 1] Spawn Buildings
          (if (`self.Spawn Right (Y+)`) :!label _label
            (`self.Building Placement` _outhit _output_2 _output 1.0 -90.0 _current_point))
          (if (`self.Cut Y- (T-Junction)`)
            (if (not _returnvalue_16)
              (if (`self.Spawn Left(Y-)`) :!label _label_2
                (`self.Building Placement` _outhit _output_2 _output -1.0 90.0 :!label _label_3)))
            (else
              (goto _label_2))))
        (elif (`self.Cut Y+ (T-Junction)`)
          (if _returnvalue_16
            (goto _label_3)
            (else
              (goto _label)))
          (else
            (goto _label))))
      ;[1 0.862 0.1944] Tile Rotation
      (`SceneComponent.K2_SetRelativeRotation` (`self.Scene`) (`KismetMathLibrary.MakeRotator` 0.0 0.0 (* (`self.Tile Rotation`) 90.0)) false false))))