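; Test tile actor that procedurally builds a floor with buildings along two opposite sides, entirely in the Construction Script.
; It adds a scaled floor mesh and two edge spawn boxes, then line-traces down over a grid on one side, mirroring hits across Y.
; BuildingVersion selects randomly rotated, height-varied houses or stacked floors, added as hierarchical instanced meshes using a seeded stream.
; The Scene component is yawed in 90-degree steps after placement.
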(fn `UserConstructionScript`
  (bind _house_scale (`self.House Scale`))
  (bind _seed (`self.Seed`))
  (bind _house_scale_2 (`self.House Scale`))
  (bind _seed_2 (`self.Seed`))
  (bind _tile_size (`self.Tile Size`))
  (bind _tile_size_2 (`self.Tile Size`))
  (bind _returnvalue (/ _tile_size_2 2.0))
  (bind _returnvalue_2 (* _tile_size_2 (`self.Spawn Width`)))
  (bind _returnvalue_3 (`KismetMathLibrary.MakeVector` _tile_size_2 _returnvalue_2 _tile_size_2))
  (bind _returnvalue_4 (* _returnvalue 100.0))
  (bind _returnvalue_5 (* (- _returnvalue (/ _returnvalue_2 2.0)) 100.0))
  (bind _returnvalue_6 (`KismetMathLibrary.MakeVector` 0.0 _returnvalue_5 _returnvalue_4))
  ;[0.04116 0.9702 1] Tile Creation
  (bind _returnvalue_7 (`AddComponent|NODE_AddStaticMeshComponent-0` :`RelativeTransform` (`KismetMathLibrary.MakeTransform` (0.0 0.0 0.0) (struct) (`KismetMathLibrary.MakeVector` _tile_size _tile_size _tile_size))))
  (`StaticMeshComponent.SetStaticMesh` _returnvalue_7 (`self.FloorMesh`))
  ;[1 0.4594 0.2061] Spawn Regions
  (`AddComponent|NODE_AddBoxComponent-0` :`RelativeTransform` (`KismetMathLibrary.MakeTransform` _returnvalue_6 (struct) _returnvalue_3))
  (`AddComponent|NODE_AddBoxComponent-1` :`RelativeTransform` (`KismetMathLibrary.MakeTransform` (`KismetMathLibrary.MakeVector` 0.0 (* -1 _returnvalue_5) _returnvalue_4) (struct) _returnvalue_3))
  ;[0.04843 1 0.9203] Set Building Mesh
  (`StaticMeshComponent.SetStaticMesh` (`self.HierarchicalInstancedStaticMesh`) (`self.Building Mesh`))
  ;[1 0.4067 0.1435] Building Spawn Grid
  (bind (_current_point _total_points _0_1_phase _poly_center) (`/Engine/ArtTools/RenderToTexture/Macros/RenderToTextureMacros.2D Grid Execution Macro` (`self.Grid Size`) (+ (`self.K2_GetActorLocation`) _returnvalue_6) (`self.House Tile X`) (`self.House Tile Y`))
    (:`Per Poly Execution`
      (bind _outhit (`KismetSystemLibrary.LineTraceSingle` :`Start` _poly_center :`End` (`KismetMathLibrary.MakeVector` (.x _poly_center) (.y _poly_center) (- (.z _poly_center) (* (`self.Tile Size`) 60.0))) :`TraceChannel` "TraceTypeQuery1" :`bIgnoreSelf` false :`DrawTime` 0.1))
      ;[0.6719 0 0.01283] SWITCH
      (switch `int` (`self.Building Version`)
        (:`0`
          (bind (_bblockinghit _binitialoverlap _time _distance _location _impactpoint _normal _impactnormal) (`GameplayStatics.BreakHitResult` _outhit))
          ;[0.07005 0.9303 1] Place Houses at Points. Rotation at random 90degree steps.
          (if _bblockinghit
            (`InstancedStaticMeshComponent.AddInstance` (`self.HierarchicalInstancedStaticMesh`) (`KismetMathLibrary.MakeTransform` (- _impactpoint (`self.K2_GetActorLocation`)) (`KismetMathLibrary.MakeRotator` (.roll (`KismetMathLibrary.MakeRotFromZX` _impactnormal (`SceneComponent.GetForwardVector` (`self.HierarchicalInstancedStaticMesh`)))) (.pitch (`KismetMathLibrary.MakeRotFromZX` _impactnormal (`SceneComponent.GetForwardVector` (`self.HierarchicalInstancedStaticMesh`)))) (+ (.yaw (`KismetMathLibrary.MakeRotFromZX` _impactnormal (`SceneComponent.GetForwardVector` (`self.HierarchicalInstancedStaticMesh`)))) (* (`KismetMathLibrary.RandomIntegerInRangeFromStream` 0 3 _seed_2) 90.0))) (`KismetMathLibrary.MakeVector` _house_scale_2 _house_scale_2 (* _house_scale_2 (`KismetMathLibrary.RandomFloatInRangeFromStream` (`self.Height Random Min`) (`self.Height Random Max`) _seed_2)))))
            (if _bblockinghit
              (`InstancedStaticMeshComponent.AddInstance` (`self.HierarchicalInstancedStaticMesh`) (`KismetMathLibrary.MakeTransform` (- (`KismetMathLibrary.MakeVector` (.x _impactpoint) (+ (.y _impactpoint) (* (.y _returnvalue_6) -2.0)) (.z _impactpoint)) (`self.K2_GetActorLocation`)) (`KismetMathLibrary.MakeRotator` (.roll (`KismetMathLibrary.MakeRotFromZX` _impactnormal (`SceneComponent.GetForwardVector` (`self.HierarchicalInstancedStaticMesh`)))) (.pitch (`KismetMathLibrary.MakeRotFromZX` _impactnormal (`SceneComponent.GetForwardVector` (`self.HierarchicalInstancedStaticMesh`)))) (+ (.yaw (`KismetMathLibrary.MakeRotFromZX` _impactnormal (`SceneComponent.GetForwardVector` (`self.HierarchicalInstancedStaticMesh`)))) (* (`KismetMathLibrary.RandomIntegerInRangeFromStream` 0 3 _seed) 90.0))) (`KismetMathLibrary.MakeVector` _house_scale _house_scale (* _house_scale (`KismetMathLibrary.RandomFloatInRangeFromStream` (`self.Height Random Min`) (`self.Height Random Max`) _seed)))))
              ;[0.1669 1 0.4103] Tile Rotation
              (`SceneComponent.K2_SetRelativeRotation` (`self.Scene`) (`KismetMathLibrary.MakeRotator` 0.0 0.0 (* (`self.Rotation`) 90.0)) false false :!label _label))))
        (:`1`
          (bind (_bblockinghit_2 _binitialoverlap_2 _time_2 _distance_2 _location_2 _impactpoint_2) (`GameplayStatics.BreakHitResult` _outhit))
          ;[0.2395 1 0.9901] Stacked Houses Y+
          (if _bblockinghit_2
            (bind _returnvalue_8 (`KismetMathLibrary.MakeVector` (.x (- _impactpoint_2 (`self.K2_GetActorLocation`))) (.y (- _impactpoint_2 (`self.K2_GetActorLocation`))) (+ (.z (- _impactpoint_2 (`self.K2_GetActorLocation`))) 50.0)))
            (`InstancedStaticMeshComponent.AddInstance` (`self.HierarchicalInstancedStaticMesh`) (`KismetMathLibrary.MakeTransform` _returnvalue_8 (struct :`Yaw` -90.0)))
            (for _index (range (+ (`KismetMathLibrary.RandomIntegerInRangeFromStream` 0 (`self.Max Floors`) (`self.Seed`)) 1))
              (`InstancedStaticMeshComponent.AddInstance` (`self.HierarchicalInstancedStaticMesh`) (`KismetMathLibrary.MakeTransform` (`KismetMathLibrary.MakeVector` (.x _returnvalue_8) (.y _returnvalue_8) (+ (.z _returnvalue_8) (* (+ _index 1) 110.0))) (struct :`Yaw` -90.0)))
              (bind (_bblockinghit_3 _binitialoverlap_3 _time_3 _distance_3 _location_3 _impactpoint_3) (`GameplayStatics.BreakHitResult` _outhit))
              ;[0.2395 1 0.9901] Stacked Houses Y-
              (if _bblockinghit_3
                (bind _returnvalue_9 (`KismetMathLibrary.MakeVector` (.x (- _impactpoint_3 (`self.K2_GetActorLocation`))) (* (.y (- _impactpoint_3 (`self.K2_GetActorLocation`))) -1.0) (+ (.z (- _impactpoint_3 (`self.K2_GetActorLocation`))) 50.0)))
                (`InstancedStaticMeshComponent.AddInstance` (`self.HierarchicalInstancedStaticMesh`) (`KismetMathLibrary.MakeTransform` _returnvalue_9 (struct :`Yaw` 90.0) (1.0 1.0 1.0)))
                (for _index_2 (range (+ (`KismetMathLibrary.RandomIntegerInRangeFromStream` 0 (`self.Max Floors`) (`self.Seed`)) 1))
                  (`InstancedStaticMeshComponent.AddInstance` (`self.HierarchicalInstancedStaticMesh`) (`KismetMathLibrary.MakeTransform` (`KismetMathLibrary.MakeVector` (.x _returnvalue_9) (.y _returnvalue_9) (+ (.z _returnvalue_9) (* (+ _index_2 1) 110.0))) (struct :`Yaw` 90.0)))
                  (goto _label))))))))))