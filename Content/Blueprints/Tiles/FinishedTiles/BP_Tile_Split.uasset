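; Forked road tile that commits the player to a left or right branch in the bike game.
; Overlap triggers block lane changes, push the player out of the middle lane by comparing raw power readings, and turn them in two 45-degree steps.
; The first bend queues floor tiles from that branch's attach point, the second shows results, and the end hit destroys the tile.
; Construction positions triggers, optional instanced lampposts and world-space building spawns.
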(event `self.LaneLock.OnComponentBeginOverlap`
  (params (OverlappedComponent :type "PrimitiveComponent Object Reference") (OtherActor :type "Actor Object Reference") (OtherComp :type "PrimitiveComponent Object Reference") (OtherBodyIndex :type Integer) (bFromSweep :type Boolean) (SweepResult :type "HitResult Structure (by ref)"))
  (bind _asbp_player_character (cast `/Game/Blueprints/Player/BP_PlayerCharacter` OtherActor))
  (`BikeCharacter.SetLaneBlocked` _asbp_player_character true))

(event `self.GTFOthemiddlelaneyoufool.OnComponentBeginOverlap`
  (params (OverlappedComponent :type "PrimitiveComponent Object Reference") (OtherActor :type "Actor Object Reference") (OtherComp :type "PrimitiveComponent Object Reference") (OtherBodyIndex :type Integer) (bFromSweep :type Boolean) (SweepResult :type "HitResult Structure (by ref)"))
  (bind _asbp_player_character (cast `/Game/Blueprints/Player/BP_PlayerCharacter` OtherActor))
  (if (> (`BikeCharacter.GetRawPower` _asbp_player_character 4) (/ (`BikeCharacter.GetRawPower` _asbp_player_character 3) 2.0))
    (`BikeCharacter.ChangePowerLane` _asbp_player_character 2 0.0)
    (else
      (`BikeCharacter.ChangePowerLane` _asbp_player_character 0 0.0))))

(event `self.BendTriggerLeftOne.OnComponentBeginOverlap`
  (params (OverlappedComponent :type "PrimitiveComponent Object Reference") (OtherActor :type "Actor Object Reference") (OtherComp :type "PrimitiveComponent Object Reference") (OtherBodyIndex :type Integer) (bFromSweep :type Boolean) (SweepResult :type "HitResult Structure (by ref)"))
  (bind _asbp_player_character (cast `/Game/Blueprints/Player/BP_PlayerCharacter` OtherActor))
  (`BikeCharacter.Turn` _asbp_player_character -45.0 (`SceneComponent.K2_GetComponentLocation` (`self.BendTriggerLeftTwo`)))
  (bind _asbp_bike_project_game_mode_base (cast `/Game/Blueprints/Gamemodes/BP_BikeProjectGameModeBase` (`GameplayStatics.GetGameMode`)))
  (set `/Game/Blueprints/Gamemodes/BP_BikeProjectGameModeBase.NextSpawnPoint` (`SceneComponent.K2_GetComponentToWorld` (`self.AttachPointLeft`)) _asbp_bike_project_game_mode_base)
  (for _ (range 6)
    (`/Game/Blueprints/Gamemodes/BP_BikeProjectGameModeBase.Add Floor Tile` _asbp_bike_project_game_mode_base "NewEnumerator0" false)))

(event `self.BendTriggerLeftTwo.OnComponentBeginOverlap`
  (params (OverlappedComponent :type "PrimitiveComponent Object Reference") (OtherActor :type "Actor Object Reference") (OtherComp :type "PrimitiveComponent Object Reference") (OtherBodyIndex :type Integer) (bFromSweep :type Boolean) (SweepResult :type "HitResult Structure (by ref)"))
  (bind _asbp_player_character (cast `/Game/Blueprints/Player/BP_PlayerCharacter` OtherActor))
  (`BikeCharacter.Turn` _asbp_player_character -45.0 (`SceneComponent.K2_GetComponentLocation` (`self.AttachPointLeft`)))
  (bind _asbp_bike_project_game_mode_base (cast `/Game/Blueprints/Gamemodes/BP_BikeProjectGameModeBase` (`GameplayStatics.GetGameMode`)))
  (`/Game/Blueprints/Gamemodes/BP_BikeProjectGameModeBase.Show Results` _asbp_bike_project_game_mode_base))

(event `self.EndTriggerLeft.OnComponentHit`
  (params (HitComponent :type "PrimitiveComponent Object Reference") (OtherActor :type "Actor Object Reference") (OtherComp :type "PrimitiveComponent Object Reference") (NormalImpulse :type "Vector Structure") (Hit :type "HitResult Structure (by ref)"))
  (bind _asbp_player_character (cast `/Game/Blueprints/Player/BP_PlayerCharacter` OtherActor))
  (`BikeCharacter.Turn` _asbp_player_character 0.0 (`SceneComponent.K2_GetComponentLocation` (`self.AttachPointLeft`)))
  (`KismetSystemLibrary.Delay` 2.0)
  (`self.K2_DestroyActor`))

(event `self.BendTriggerRightOne.OnComponentBeginOverlap`
  (params (OverlappedComponent :type "PrimitiveComponent Object Reference") (OtherActor :type "Actor Object Reference") (OtherComp :type "PrimitiveComponent Object Reference") (OtherBodyIndex :type Integer) (bFromSweep :type Boolean) (SweepResult :type "HitResult Structure (by ref)"))
  (bind _asbp_player_character (cast `/Game/Blueprints/Player/BP_PlayerCharacter` OtherActor))
  (`BikeCharacter.Turn` _asbp_player_character 45.0 (`SceneComponent.K2_GetComponentLocation` (`self.BendTriggerRightTwo`)))
  (bind _asbp_bike_project_game_mode_base (cast `/Game/Blueprints/Gamemodes/BP_BikeProjectGameModeBase` (`GameplayStatics.GetGameMode`)))
  (set `/Game/Blueprints/Gamemodes/BP_BikeProjectGameModeBase.NextSpawnPoint` (`SceneComponent.K2_GetComponentToWorld` (`self.AttachPointRight`)) _asbp_bike_project_game_mode_base)
  (for _ (range 6)
    (`/Game/Blueprints/Gamemodes/BP_BikeProjectGameModeBase.Add Floor Tile` _asbp_bike_project_game_mode_base "NewEnumerator0" false)))

(event `self.BendTriggerRightTwo.OnComponentBeginOverlap`
  (params (OverlappedComponent :type "PrimitiveComponent Object Reference") (OtherActor :type "Actor Object Reference") (OtherComp :type "PrimitiveComponent Object Reference") (OtherBodyIndex :type Integer) (bFromSweep :type Boolean) (SweepResult :type "HitResult Structure (by ref)"))
  (bind _asbp_player_character (cast `/Game/Blueprints/Player/BP_PlayerCharacter` OtherActor))
  (`BikeCharacter.Turn` _asbp_player_character 45.0 (`SceneComponent.K2_GetComponentLocation` (`self.AttachPointRight`)))
  (bind _asbp_bike_project_game_mode_base (cast `/Game/Blueprints/Gamemodes/BP_BikeProjectGameModeBase` (`GameplayStatics.GetGameMode`)))
  (`/Game/Blueprints/Gamemodes/BP_BikeProjectGameModeBase.Show Results` _asbp_bike_project_game_mode_base))

(event `self.EndTriggerRight.OnComponentHit`
  (params (HitComponent :type "PrimitiveComponent Object Reference") (OtherActor :type "Actor Object Reference") (OtherComp :type "PrimitiveComponent Object Reference") (NormalImpulse :type "Vector Structure") (Hit :type "HitResult Structure (by ref)"))
  (bind _asbp_player_character (cast `/Game/Blueprints/Player/BP_PlayerCharacter` OtherActor))
  (`BikeCharacter.Turn` _asbp_player_character 0.0 (`SceneComponent.K2_GetComponentLocation` (`self.AttachPointRight`)))
  (`KismetSystemLibrary.Delay` 2.0)
  (`self.K2_DestroyActor`))

(fn `Make Lampposts`
  (bind _lamppost_amount (`self.Lamppost Amount`))
  (bind _lampost_01 (`self.Lampost_01`))
  (bind _lamppost_ypos (`self.Lamppost Ypos`))
  (`|ExecutionSequence`
    (:`then_0`
      (bind (_current_point _total_points _0_1_phase _poly_center) (`/Engine/ArtTools/RenderToTexture/Macros/RenderToTextureMacros.2D Grid Execution Macro` (/ 1000.0 (`KismetMathLibrary.Conv_IntToDouble` _lamppost_amount)) (`KismetMathLibrary.MakeVector` 500.0 0.0 8.0) _lamppost_amount 1)
        (:`Per Poly Execution`
          (bind _x (.x _poly_center))
          (bind _z (.z _poly_center))
          (`InstancedStaticMeshComponent.AddInstance` _lampost_01 (`KismetMathLibrary.MakeTransform` (`KismetMathLibrary.MakeVector` _x _lamppost_ypos _z)))
          (`InstancedStaticMeshComponent.AddInstance` _lampost_01 (`KismetMathLibrary.MakeTransform` (`KismetMathLibrary.MakeVector` _x (- 0.0 _lamppost_ypos) _z) (struct :`Yaw` 180.0))))))))

(fn `Preview Buildings`
  (bind _rotation (.rotation (`self.GetTransform` self)))
  (`KismetArrayLibrary.Array_Clear` (`self.worldSpawnLocation`))
  (for _array_element (`self.BuildingSpawnLocation`)
    (`KismetArrayLibrary.Array_Add` (`self.worldSpawnLocation`) (`KismetMathLibrary.MakeTransform` (+ (`KismetMathLibrary.RotateAngleAxis` (.location _array_element) (.yaw _rotation) (0.0 0.0 1.0)) (.location (`self.GetTransform` self))) (`KismetMathLibrary.ComposeRotators` _rotation (.rotation _array_element)))))
  (bind _returnvalue (`GameplayStatics.GetActorOfClass` "/Game/Blueprints/Art/BP_Buildings.BP_Buildings_C"))
  (`/Game/Blueprints/Art/BP_Buildings.Preview Buildings` _returnvalue (`self.worldSpawnLocation`)))

(fn `UserConstructionScript`
  (bind _rotation (.rotation (`self.GetTransform` self)))
  (set `self.Floor Mesh` (`self.RoadMesh`))
  (`|ExecutionSequence`
    (:`then_0`
      (if (`self.Make Lampposts Bool`)
        (`self.Make Lampposts`))
      (for _array_element (`self.BuildingSpawnLocation`)
        (`KismetArrayLibrary.Array_Add` (`self.worldSpawnLocation`) (`KismetMathLibrary.MakeTransform` (+ (`KismetMathLibrary.RotateAngleAxis` (.location _array_element) (.yaw _rotation) (0.0 0.0 1.0)) (.location (`self.GetTransform` self))) (`KismetMathLibrary.ComposeRotators` _rotation (.rotation _array_element)))))
      (set `self.BuildingSpawns` (`self.worldSpawnLocation`)))
    (:`then_1`
      (`SceneComponent.K2_SetRelativeTransform` (`self.AttachPointLeft`) (`KismetMathLibrary.MakeTransform` (1707.109985 -1700.109985 0.0) (struct :`Yaw` -90.0)) false false)
      (`SceneComponent.K2_SetRelativeTransform` (`self.AttachPointRight`) (`KismetMathLibrary.MakeTransform` (1707.109985 1700.109985 0.0) (struct :`Yaw` 90.0)) false false)
      (`SceneComponent.K2_SetRelativeTransform` (`self.BendTriggerLeftOne`) (`KismetMathLibrary.MakeTransform` (+ (`KismetMathLibrary.RotateAngleAxis` (55.0 0.0 0.0) 67.5 (0.0 0.0 1.0)) (931.655029 -165.0 0.0)) (struct :`Yaw` 67.5)) false false)
      (`SceneComponent.K2_SetRelativeTransform` (`self.BendTriggerRightOne`) (`KismetMathLibrary.MakeTransform` (+ (`KismetMathLibrary.RotateAngleAxis` (55.0 0.0 0.0) -67.5 (0.0 0.0 1.0)) (931.655029 165.0 0.0)) (struct :`Yaw` -67.5)) false false)
      (`SceneComponent.K2_SetRelativeTransform` (`self.BendTriggerLeftTwo`) (`KismetMathLibrary.MakeTransform` (+ (`KismetMathLibrary.RotateAngleAxis` (165.0 0.0 0.0) 22.5 (0.0 0.0 1.0)) (1542.109985 -775.452026 0.0)) (struct :`Yaw` 22.5)) false false)
      (`SceneComponent.K2_SetRelativeTransform` (`self.BendTriggerRightTwo`) (`KismetMathLibrary.MakeTransform` (+ (`KismetMathLibrary.RotateAngleAxis` (165.0 0.0 0.0) -22.5 (0.0 0.0 1.0)) (1542.109985 775.452026 0.0)) (struct :`Yaw` -22.5)) false false))))