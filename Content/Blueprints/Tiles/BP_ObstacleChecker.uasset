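; BP_ObstacleChecker is a tile obstacle that tests the player character's power when hit.
; On Hit, it compares the player's raw power at fixed index 4 against the raw power for its Lane.
; If the index 4 value is not greater, it decrements PlayerHealth in BikeGameInstance.
; The obstacle destroys itself after either outcome.
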(event `self.ReceiveBeginPlay`)

(event `self.ReceiveActorBeginOverlap`
  (params (OtherActor :type "Actor Object Reference")))

(event `self.ReceiveHit`
  (params (MyComp :type "PrimitiveComponent Object Reference") (Other :type "Actor Object Reference") (OtherComp :type "PrimitiveComponent Object Reference") (bSelfMoved :type Boolean) (HitLocation :type "Vector Structure") (HitNormal :type "Vector Structure") (NormalImpulse :type "Vector Structure") (Hit :type "HitResult Structure (by ref)"))
  (bind _asbp_player_character (cast `/Game/Blueprints/Player/BP_PlayerCharacter` Other))
  (if (> (`BikeCharacter.GetRawPower` _asbp_player_character 4) (`BikeCharacter.GetRawPower` _asbp_player_character (`self.Lane`)))
    (`self.K2_DestroyActor`)
    (else
      ;[1 1 1] If Player isnt the Correct Power Consquence (lower health?) /Annabelle
      (bind _asbike_game_instance (cast `BikeGameInstance` (`GameplayStatics.GetGameInstance`)))
      (bind _result (`/Engine/EditorBlueprintResources/StandardMacros.DecrementInt` (`BikeGameInstance.PlayerHealth` _asbike_game_instance))
        (:`  `
          (`BikeGameInstance.SetPlayerHealth` _asbike_game_instance _result)
          (`self.K2_DestroyActor`))))))

(fn `UserConstructionScript`)