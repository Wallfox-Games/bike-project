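; BP_PowerUpHealth is a health pickup that randomly appears as either a ham or a burger mesh, chosen in the construction script.
; When its sphere is overlapped by BP_PlayerCharacter, it calls IncPlayerHealth on that character's BP_BikePlayerController.
; It then disables collision on the static mesh, but does not hide or destroy the actor or disable the sphere in this graph.
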(event `self.Sphere.OnComponentBeginOverlap`
  (params (OverlappedComponent :type "PrimitiveComponent Object Reference") (OtherActor :type "Actor Object Reference") (OtherComp :type "PrimitiveComponent Object Reference") (OtherBodyIndex :type Integer) (bFromSweep :type Boolean) (SweepResult :type "HitResult Structure (by ref)"))
  (bind _asbp_player_character (cast `/Game/Blueprints/Player/BP_PlayerCharacter` OtherActor))
  (bind _asbp_bike_player_controller (cast `/Game/Blueprints/Player/BP_BikePlayerController` (`Pawn.GetController` _asbp_player_character)))
  (`BikeProjectPlayerController.IncPlayerHealth` _asbp_bike_player_controller false)
  (`PrimitiveComponent.SetCollisionEnabled` (`self.StaticMesh`) "NoCollision"))

(fn `UserConstructionScript`
  (bind _staticmesh (`self.StaticMesh`))
  (if (`KismetMathLibrary.RandomBool`)
    (`StaticMeshComponent.SetStaticMesh` _staticmesh "/Game/Meshes/Gameplay_Props/SM_ham_01.SM_ham_01")
    (else
      (`StaticMeshComponent.SetStaticMesh` _staticmesh "/Game/Meshes/Gameplay_Props/SM_burger.SM_burger"))))