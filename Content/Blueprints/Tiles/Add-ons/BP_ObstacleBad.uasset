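; BP_ObstacleBad is a tile add-on obstacle that penalizes the player in a bike game when hit.
; The construction script randomly assigns one of two construction-work Blueprints to its DestructibleMesh child actor.
; Its OnHit override, gated by ActivatedOnHit, passes false to the bike player controller's ChangeComboMeter and PlayerHit, then calls the parent implementation.
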(event `self.ReceiveBeginPlay`)

(event `self.ReceiveActorBeginOverlap`
  (params (OtherActor :type "Actor Object Reference")))

(event `self.ReceiveHit`
  (params (MyComp :type "PrimitiveComponent Object Reference") (Other :type "Actor Object Reference") (OtherComp :type "PrimitiveComponent Object Reference") (bSelfMoved :type Boolean) (HitLocation :type "Vector Structure") (HitNormal :type "Vector Structure") (NormalImpulse :type "Vector Structure") (Hit :type "HitResult Structure (by ref)")))

(fn `On Hit`
  (if (not (`self.ActivatedOnHit`))
    (bind _asbp_bike_player_controller (cast `/Game/Blueprints/Player/BP_BikePlayerController` (`GameplayStatics.GetPlayerController` 0)))
    (`BikeProjectPlayerController.ChangeComboMeter` _asbp_bike_player_controller false)
    (`BikeProjectPlayerController.PlayerHit` _asbp_bike_player_controller false)
    (`parent.On Hit`)))

(fn `UserConstructionScript`
  (bind _destructiblemesh (`self.DestructibleMesh`))
  (if (`KismetMathLibrary.RandomBool`)
    (`ChildActorComponent.SetChildActorClass` _destructiblemesh "/Game/Blueprints/Art/Destructibles/BP_Construction_Work_01.BP_Construction_Work_01_C")
    (else
      (`ChildActorComponent.SetChildActorClass` _destructiblemesh "/Game/Blueprints/Art/Destructibles/BP_Construction_Work_02.BP_Construction_Work_02_C"))))