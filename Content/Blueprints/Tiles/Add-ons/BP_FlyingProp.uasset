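; BP_FlyingProp is a tile add-on actor that animates a prop hovering around its spawn point.
; BeginPlay stores the start location and picks a random signed movement multiplier, varying size and direction per instance.
; Tick uses sine and cosine of elapsed time to loop the actor in the world Y-Z plane and sway its yaw around 180 degrees, forcing unit scale.
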(event `self.ReceiveBeginPlay`
  (bind _returnvalue (`KismetMathLibrary.RandomFloatInRange` 10.0 70.0))
  (`|ExecutionSequence`
    (:`then_0`
      (set `self.Root Location` (`self.K2_GetActorLocation`)))
    (:`then_1`
      (if (`KismetMathLibrary.RandomBool`)
        (set `self.Movement Multiplier` _returnvalue)
        (else
          (set `self.Movement Multiplier` (* _returnvalue -1.0)))))))

(event `self.ReceiveTick`
  (params (DeltaSeconds :type "Float (single-precision)"))
  (bind _movement_multiplier (`self.Movement Multiplier`))
  (bind _output_get (set `self.TimeElapsed` (+ DeltaSeconds (`self.TimeElapsed`))))
  (bind _returnvalue (`KismetMathLibrary.Sin` _output_get))
  (`self.K2_SetActorTransform` (`KismetMathLibrary.MakeTransform` (+ (`KismetMathLibrary.MakeVector` 0.0 0.0 (* (`KismetMathLibrary.Cos` _output_get) _movement_multiplier)) (`self.Root Location`) (* (`KismetMathLibrary.GetRightVector` (struct)) (* _returnvalue _movement_multiplier))) (`KismetMathLibrary.MakeRotator` 0.0 0.0 (+ (* _returnvalue _movement_multiplier) 180.0)))))

(fn `UserConstructionScript`)