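; Template Blueprint for a bent road tile in a bike game, with triggers, attach point and building spawns.
; Construction script places BendTrigger, EndTrigger and AttachPoint from the bend Angle and converts building spawn transforms to world space.
; BendTrigger turns the player once by Angle; EndTrigger calls Turn with zero angle, requests the next tile from the game mode, then destroys this one after a delay.
; PreviewBuildings sends recomputed spawns to BP_Buildings.
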(event `self.ReceiveBeginPlay`
  (set `self.Turned` false))

(event `self.EndTrigger.OnComponentBeginOverlap`
  (params (OverlappedComponent :type "PrimitiveComponent Object Reference") (OtherActor :type "Actor Object Reference") (OtherComp :type "PrimitiveComponent Object Reference") (OtherBodyIndex :type Integer) (bFromSweep :type Boolean) (SweepResult :type "HitResult Structure (by ref)"))
  (bind _asbp_player_character (cast `/Game/Blueprints/Player/BP_PlayerCharacter` OtherActor))
  (`BikeCharacter.Turn` _asbp_player_character 0.0 (`SceneComponent.K2_GetComponentLocation` (`self.AttachPoint`)))
  (bind _asbp_bike_project_game_mode_base (cast `/Game/Blueprints/Gamemodes/BP_BikeProjectGameModeBase` (`GameplayStatics.GetGameMode`)))
  (`/Game/Blueprints/Gamemodes/BP_BikeProjectGameModeBase.Next Floor Tile` _asbp_bike_project_game_mode_base)
  (`KismetSystemLibrary.Delay` 2.0)
  (`self.K2_DestroyActor`))

(event `self.BendTrigger.OnComponentBeginOverlap`
  (params (OverlappedComponent :type "PrimitiveComponent Object Reference") (OtherActor :type "Actor Object Reference") (OtherComp :type "PrimitiveComponent Object Reference") (OtherBodyIndex :type Integer) (bFromSweep :type Boolean) (SweepResult :type "HitResult Structure (by ref)"))
  (bind _asbp_player_character (cast `/Game/Blueprints/Player/BP_PlayerCharacter` OtherActor))
  (if (not (`self.Turned`))
    (`BikeCharacter.Turn` _asbp_player_character (`self.Angle`) (`SceneComponent.K2_GetComponentLocation` (`self.AttachPoint`)))
    (set `self.Turned` true)))

(fn `Preview Buildings`
  (bind _rotation (.rotation (`self.GetTransform` self)))
  (`KismetArrayLibrary.Array_Clear` (`self.worldSpawnLocation`))
  (for _array_element (`self.BuildingSpawnLocation`)
    (`KismetArrayLibrary.Array_Add` (`self.worldSpawnLocation`) (`KismetMathLibrary.MakeTransform` (+ (`KismetMathLibrary.RotateAngleAxis` (.location _array_element) (.yaw _rotation) (0.0 0.0 1.0)) (.location (`self.GetTransform` self))) (`KismetMathLibrary.ComposeRotators` _rotation (.rotation _array_element)))))
  (bind _returnvalue (`GameplayStatics.GetActorOfClass` "/Game/Blueprints/Art/BP_Buildings.BP_Buildings_C"))
  (`/Game/Blueprints/Art/BP_Buildings.Preview Buildings` _returnvalue (`self.worldSpawnLocation`)))

(fn `UserConstructionScript`
  (bind _angle (`self.Angle`))
  (bind _returnvalue (`KismetMathLibrary.MakeRotator` 0.0 0.0 _angle))
  (bind _rotation (.rotation (`self.GetTransform` self)))
  (bind _returnvalue_2 (+ (`KismetMathLibrary.RotateAngleAxis` (500.0 0.0 0.0) _angle (0.0 0.0 1.0)) (500.0 0.0 0.0)))
  (`|ExecutionSequence`
    (:`then_0`
      (set `self.Floor Mesh` (`self.RoadMesh`))
      (for _array_element (`self.BuildingSpawnLocation`)
        (`KismetArrayLibrary.Array_Add` (`self.worldSpawnLocation`) (`KismetMathLibrary.MakeTransform` (+ (`KismetMathLibrary.RotateAngleAxis` (.location _array_element) (.yaw _rotation) (0.0 0.0 1.0)) (.location (`self.GetTransform` self))) (`KismetMathLibrary.ComposeRotators` _rotation (.rotation _array_element)))))
      (set `self.BuildingSpawns` (`self.worldSpawnLocation`)))
    (:`then_1`
      (`SceneComponent.K2_SetRelativeTransform` (`self.EndTrigger`) (`KismetMathLibrary.MakeTransform` (+ _returnvalue_2 (0.0 0.0 200.0)) _returnvalue (1.0 5.0 10.0)) false false)
      (`SceneComponent.K2_SetRelativeTransform` (`self.AttachPoint`) (`KismetMathLibrary.MakeTransform` (- _returnvalue_2 (`KismetMathLibrary.RotateAngleAxis` (7.0 0.0 0.0) _angle (0.0 0.0 1.0))) _returnvalue) false false))
    (:`then_2`
      (`SceneComponent.K2_SetRelativeTransform` (`self.BendTrigger`) (`KismetMathLibrary.MakeTransform` (500.0 0.0 0.0) (`KismetMathLibrary.MakeRotator` 0.0 0.0 (+ (/ (`self.Angle`) 2.0) 90.0))) false false))))