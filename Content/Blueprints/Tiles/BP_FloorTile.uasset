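; Floor tile segment for an endless bike game that picks a random tile child actor from BP_LevelDatabaseActor, avoiding the previous type.
; Construction adds good, bad or health obstacles across three lanes (bad fills two, leaving one free) and optional flying props.
; Separate functions place buildings and set lane materials.
; The player crossing EndTrigger requests the next tile from the game mode, then the tile removes itself and its buildings after a delay.
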(event `self.ReceiveBeginPlay`
  (bind _returnvalue (`GameplayStatics.GetActorOfClass` "/Game/Blueprints/Art/BP_Buildings.BP_Buildings_C"))
  (set `self.Building Reference` _returnvalue))

(event `self.EndTrigger.OnComponentBeginOverlap`
  (params (OverlappedComponent :type "PrimitiveComponent Object Reference") (OtherActor :type "Actor Object Reference") (OtherComp :type "PrimitiveComponent Object Reference") (OtherBodyIndex :type Integer) (bFromSweep :type Boolean) (SweepResult :type "HitResult Structure (by ref)"))
  (cast `/Game/Blueprints/Player/BP_PlayerCharacter` OtherActor)
  (bind _asbp_bike_project_game_mode_base (cast `/Game/Blueprints/Gamemodes/BP_BikeProjectGameModeBase` (`GameplayStatics.GetGameMode`)))
  (`/Game/Blueprints/Gamemodes/BP_BikeProjectGameModeBase.Next Floor Tile` _asbp_bike_project_game_mode_base)
  (`KismetSystemLibrary.Delay` 2.0)
  (`self.Destroy Self`))

(fn `Destroy Building Instances`
  (`/Game/Blueprints/Art/BP_Buildings.Destroy Buildings` (`self.Building Reference`)))

(fn `Destroy Self`
  (bind _asbp_bike_project_game_mode_base (cast `/Game/Blueprints/Gamemodes/BP_BikeProjectGameModeBase` (`GameplayStatics.GetGameMode`)))
  (`KismetArrayLibrary.Array_Remove` (`/Game/Blueprints/Gamemodes/BP_BikeProjectGameModeBase.Tile Info Array` _asbp_bike_project_game_mode_base))
  (`self.Destroy Building Instances`)
  (`self.K2_DestroyActor`))

(fn `Get Tile Class`
  (returns (`Tile Class` :type "Actor Class Reference") (`Tile Type` :type Integer))
  (return (`self.Tile Class`) (`self.New Tile Type`)))

(fn `GetAttachTransform`
  (returns (AttachTransform :type "Transform Structure"))
  (return (`SceneComponent.K2_GetComponentToWorld` (`self.AttachPoint`))))

(fn `Set Lanes`
  (params (`Obstacle Type` :type "/Game/Blueprints/Tiles/Add-ons/E_ObstacleType Enum" :default "NewEnumerator0") (`Lane Array` :type "Array of Integer"))
  (bind _output (`|GetArrayItem` `Lane Array`))
  (bind _asbp_tile_class (cast `/Game/Blueprints/Tiles/BP_Tile_Class` (`ChildActorComponent.ChildActor` (`self.TileChild`))))
  (switch `/Game/Blueprints/Tiles/Add-ons/E_ObstacleType` `Obstacle Type`
    (:`NewEnumerator1`
      (`/Game/Blueprints/Tiles/BP_Tile_Class.Set Lane Material` _asbp_tile_class _output null))
    (:`NewEnumerator2`
      (`/Game/Blueprints/Tiles/BP_Tile_Class.Set Lane Material` _asbp_tile_class _output null)
      (`/Game/Blueprints/Tiles/BP_Tile_Class.Set Lane Material` _asbp_tile_class (`|GetArrayItem` `Lane Array` 1) null))
    (:`NewEnumerator4`
      (`/Game/Blueprints/Tiles/BP_Tile_Class.Set Lane Material` _asbp_tile_class _output null))))

(fn `SetSpawnArray`
  (`|ExecutionSequence`
    (:`then_0`
      (set `self.SpawnPoints` (`|MakeArray` (`SceneComponent.GetRelativeTransform` (`self.ObstacleSpawnL`)) (`SceneComponent.GetRelativeTransform` (`self.ObstacleSpawnC`)) (`SceneComponent.GetRelativeTransform` (`self.ObstacleSpawnR`)))))
    (:`then_1`
      (set `self.FlyingPoints` (`|MakeArray` (`SceneComponent.GetRelativeTransform` (`self.FlyingSpawnL`)) (`SceneComponent.GetRelativeTransform` (`self.FlyingSpawnM`)) (`SceneComponent.GetRelativeTransform` (`self.FlyingSpawnH`)))))))

(fn `Spawn Buildings`
  (bind _asbp_tile_class (cast `/Game/Blueprints/Tiles/BP_Tile_Class` (`ChildActorComponent.ChildActor` (`self.TileChild`))))
  (bind _returnvalue (`GameplayStatics.GetActorOfClass` "/Game/Blueprints/Art/BP_Buildings.BP_Buildings_C"))
  (`/Game/Blueprints/Art/BP_Buildings.new_placeBuildings` _returnvalue (`/Game/Blueprints/Tiles/BP_Tile_Class.BuildingSpawns` _asbp_tile_class)))

(fn `Spawn Flying Object`
  (`AddComponent|NODE_AddChildActorComponent-4` :`RelativeTransform` (`|GetArrayItem` (`self.FlyingPoints`) (`KismetMathLibrary.RandomInteger` 3))))

(fn `SpawnObstacleBad`
  (bind _output_get (set `self.Random Lane` (`KismetMathLibrary.RandomInteger` 3)))
  (for (_array_element _array_index) (`self.SpawnPoints`)
    (if (!= _array_index _output_get)
      (`KismetArrayLibrary.Array_Add` (`self.Obstacle Lanes`) _array_index)
      (`AddComponent|NODE_AddChildActorComponent-2` :`RelativeTransform` _array_element))))

(fn `SpawnObstacleGood`
  (bind _output_get (set `self.Random Lane` (`KismetMathLibrary.RandomInteger` 3)))
  (for (_array_element _array_index) (`self.SpawnPoints`)
    (if (== _array_index _output_get)
      (`KismetArrayLibrary.Array_Add` (`self.Obstacle Lanes`) _array_index)
      (`AddComponent|NODE_AddChildActorComponent-0` :`RelativeTransform` _array_element))))

(fn `SpawnObstacleHealth`
  (bind _output_get (set `self.Random Lane` (`KismetMathLibrary.RandomInteger` 3)))
  (for (_array_element _array_index) (`self.SpawnPoints`)
    (if (== _array_index _output_get)
      (`KismetArrayLibrary.Array_Add` (`self.Obstacle Lanes`) _array_index)
      (`AddComponent|NODE_AddChildActorComponent-3` :`RelativeTransform` _array_element))))

(fn `UserConstructionScript`
  (bind _new_tile_type (`self.New Tile Type`))
  (bind _previous_tile_type (`self.Previous Tile Type`))
  (`self.SetSpawnArray`)
  (bind _returnvalue (`GameplayStatics.GetActorOfClass` "/Game/Blueprints/Art/BP_LevelDatabaseActor.BP_LevelDatabaseActor_C"))
  (set `self.New Tile Type` _previous_tile_type)
  (while (== _new_tile_type _previous_tile_type)
    (bind _tiles (`/Game/Blueprints/Art/BP_LevelDatabaseActor.Tiles` _returnvalue))
    (set `self.New Tile Type` (`KismetMathLibrary.RandomIntegerInRange` 0 (- (`KismetArrayLibrary.Array_Length` _tiles) 1))))
  (bind _output_get (set `self.Tile Class` (`|GetArrayItem` _tiles _new_tile_type)))
  (`ChildActorComponent.SetChildActorClass` (`self.TileChild`) _output_get)
  (if (`self.FlyingProp`)
    (`self.Spawn Flying Object`))
  (switch `/Game/Blueprints/Tiles/Add-ons/E_ObstacleType` (`self.Obstacle Spawn`)
    (:`NewEnumerator1`
      (`self.SpawnObstacleGood`))
    (:`NewEnumerator2`
      (`self.SpawnObstacleBad`))
    (:`NewEnumerator4`
      (`self.SpawnObstacleHealth`))))