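; Game mode Blueprint that builds the floor out of tiles, laying down an initial ten at BeginPlay.
; BeginPlay resets the tile count, then calls NextFloorTile in a loop.
; NextFloorTile overrides a parent function and picks one of two enum tile types by count modulo three, giving one variant in every three, before passing it to AddFloorTile.
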(event `self.ReceiveBeginPlay`
  (`parent.ReceiveBeginPlay`)
  (set `self.Current Tile Count` 0)
  (for _ (range 10)
    (`self.Next Floor Tile`)))

(fn `Next Floor Tile`
  (`parent.Next Floor Tile`)
  (if (== (mod (`self.Current Tile Count`) 3) 1)
    (`self.Add Floor Tile` "NewEnumerator1")
    (else
      (`self.Add Floor Tile` "NewEnumerator0"))))

(fn `UserConstructionScript`
  (`parent.UserConstructionScript`))