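; Game mode for the bike project that builds the track by chaining floor tiles, laying ten at BeginPlay.
; AddFloorTile spawns each tile at the previous tile's attach transform and has the level's BP_Buildings actor place buildings there.
; A running tile count gives every third tile a different obstacle-spawn setting, except while the player character's tutorial state is active.
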(event `self.ReceiveBeginPlay`
  (bind _returnvalue (`GameplayStatics.GetActorOfClass` "/Game/Blueprints/Art/BP_Buildings.BP_Buildings_C"))
  (set `self.Building Reference` _returnvalue)
  (set `self.Current Tile Count` 0)
  (for _ (range 10)
    (`self.Add Floor Tile`)))

(event `self.ReceiveTick`
  (params (DeltaSeconds :type "Float (single-precision)")))

(fn `Add Floor Tile`
  (bind _nextspawnpoint (`self.NextSpawnPoint`))
  (`self.Increment Tile Count`)
  (bind _asbp_player_character (cast `/Game/Blueprints/BP_PlayerCharacter` (`GameplayStatics.GetPlayerPawn` 0)))
  (if (`BikeCharacter.GetTutorialState` _asbp_player_character)
    (set `self.Obstacle Spawn` "NewEnumerator0")
    (elif (== (mod (`self.Current Tile Count`) 3) 1)
      (set `self.Obstacle Spawn` "NewEnumerator1")
      (else
        (set `self.Obstacle Spawn` "NewEnumerator0"))))
  (bind _returnvalue (`|SpawnActorFromClass` "/Game/Blueprints/BP_FloorTile.BP_FloorTile_C" _nextspawnpoint "Undefined" "OverrideRootScale" null (`self.Obstacle Spawn`) null))
  (`self.Spawn Buildings` _nextspawnpoint)
  (bind _attachtransform (`/Game/Blueprints/BP_FloorTile.GetAttachTransform` _returnvalue))
  (set `self.NextSpawnPoint` _attachtransform))

(fn `Increment Tile Count`
  (set `self.Current Tile Count` (+ (`self.Current Tile Count`) 1)))

(fn `Spawn Buildings`
  (params (`Spawn Transform` :type "Transform Structure"))
  (`/Game/Blueprints/Art/BP_Buildings.Place Buildings` (`self.Building Reference`) `Spawn Transform`))

(fn `UserConstructionScript`)